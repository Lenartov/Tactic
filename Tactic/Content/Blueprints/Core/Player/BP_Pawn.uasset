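; BP_Pawn is a player camera pawn with spring-arm zoom, planar movement and yaw rotation.
; Enhanced Input actions only update desired targets: clamped arm length, location offset along the pawn's forward and right vectors, and stepped yaw.
; Tick eases arm length, actor location and rotation toward those targets with separate interp speeds, moving without sweep, so there is no collision check.
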(event Input|EnhancedActionEvents|EnhancedInputActionIA_CameraZoom
  (params (ActionValue :type Float%20%28double-precision%29) (ElapsedSeconds :type Float%20%28double-precision%29) (TriggeredSeconds :type Float%20%28double-precision%29) (InputAction :type Input%20Action%20Object%20Reference :default "/Game/Blueprints/Core/Input/IA_CameraZoom.IA_CameraZoom"))
  (Variables|Default|SetZoomDesired (Math|Float|Clamp(Float) (+ (* ActionValue (Variables|Default|GetZoomSpeed)) (Variables|Default|GetZoomDesired)) (Variables|Default|GetMinZoom) (Variables|Default|GetMaxZoom))))

(event Input|EnhancedActionEvents|EnhancedInputActionIA_RotateLeft
  (params (ActionValue :type Boolean) (ElapsedSeconds :type Float%20%28double-precision%29) (TriggeredSeconds :type Float%20%28double-precision%29) (InputAction :type Input%20Action%20Object%20Reference :default "/Game/Blueprints/Core/Input/IA_RotateLeft.IA_RotateLeft"))
  (Variables|Default|SetRotateDesired (Math|Rotator|CombineRotators (Variables|Default|GetRotateDesired) (Math|Rotator|MakeRotator 0.0 0.0 (Variables|Default|GetRotationSpeed)))))

(event Input|EnhancedActionEvents|EnhancedInputActionIA_RotateRight
  (params (ActionValue :type Boolean) (ElapsedSeconds :type Float%20%28double-precision%29) (TriggeredSeconds :type Float%20%28double-precision%29) (InputAction :type Input%20Action%20Object%20Reference :default "/Game/Blueprints/Core/Input/IA_RotateRight.IA_RotateRight"))
  (Variables|Default|SetRotateDesired (Math|Rotator|CombineRotators (Variables|Default|GetRotateDesired) (Math|Rotator|MakeRotator 0.0 0.0 (- 0.0 (Variables|Default|GetRotationSpeed))))))

(event Input|EnhancedActionEvents|EnhancedInputActionIA_CameraMovement
  (params (ActionValue :type Vector%202D%20Structure) (ElapsedSeconds :type Float%20%28double-precision%29) (TriggeredSeconds :type Float%20%28double-precision%29) (InputAction :type Input%20Action%20Object%20Reference :default "/Game/Blueprints/Core/Input/IA_CameraMovement.IA_CameraMovement"))
  (bind _movementspeed (Variables|Default|GetMovementSpeed))
  (bind _returnvalue (* ActionValue _movementspeed))
  (bind (_x _y) (Math|Vector|BreakVector _returnvalue))
  (Variables|Default|SetLocationDesired (+ (Variables|Default|GetLocationDesired) (* (Transformation|GetActorForwardVector) _x) (* (Transformation|GetActorRightVector) _y))))

(event EventTick
  (params (DeltaSeconds :type Float%20%28single-precision%29))
  (bind _springarm (Variables|Default|GetSpringArm))
  (Variables|/Script/Engine.SpringArmComponent|SetTargetArmLength _springarm (Math|Interpolation|FInterpTo (Variables|/Script/Engine.SpringArmComponent|GetTargetArmLength _springarm) (Variables|Default|GetZoomDesired) DeltaSeconds (Variables|Default|GetZoomInter)))
  (Transformation|SetActorLocation (Math|Interpolation|VInterpTo (Transformation|GetActorLocation) (Variables|Default|GetLocationDesired) DeltaSeconds (Variables|Default|GetMovementInter)) false false)
  (Transformation|SetActorRotation (Math|Interpolation|RInterpTo (Transformation|GetActorRotation) (Variables|Default|GetRotateDesired) DeltaSeconds (Variables|Default|GetRotationInter))))

(event EventBeginPlay
  (Variables|Default|SetZoomDesired (Variables|/Script/Engine.SpringArmComponent|GetTargetArmLength (Variables|Default|GetSpringArm)))
  (Variables|Default|SetLocationDesired (Transformation|GetActorLocation))
  (Variables|Default|SetRotateDesired (Transformation|GetActorRotation)))

(fn ConstructionScript)