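; Player input actor for grid-based tactics that manages hovered and selected tiles and units.
; Each tick it resolves the hovered unit or tile under the cursor and updates its highlight.
; Left and right clicks execute swappable spawned action actors on the hovered tile, repeating as a held button drags across tiles.
; Grid and combat system events refresh selection, follow unit turns, clear actions and toggle the combat widget.
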(event Custom|OnHoveredTileChanged
  (bind _selectedactionleftclick (Variables|Default|GetSelectedActionLeftClick))
  (bind _selectedactionrightclick (Variables|Default|GetSelectedActionRightClick))
  (bind _hoveredtile (Variables|Default|GetHoveredTile))
  (Utilities|FlowControl|Sequence
    (:then_0
      (Utilities|IsValid _selectedactionleftclick
        (:Is%20Valid
          (Default|ExecuteHovered _selectedactionleftclick _hoveredtile)
          (if (Variables|Default|GetIsLeftPressed)
            (Default|Execute (Variables|Default|GetSelectedActionLeftClick) (Variables|Default|GetHoveredTile))))))
    (:then_1
      (Utilities|IsValid _selectedactionrightclick
        (:Is%20Valid
          (Default|ExecuteHovered _selectedactionrightclick _hoveredtile)
          (if (Variables|Default|GetIsRightPressed)
            (Default|Execute (Variables|Default|GetSelectedActionRightClick) (Variables|Default|GetHoveredTile))))))))

(event EventBeginPlay
  (bind _returnvalue (Actor|GetActorOfClass "/Game/Blueprints/Core/Grid/BP_Grid.BP_Grid_C"))
  (bind _output_get (Variables|Default|SetGrid _returnvalue))
  (EventDispatchers|BindEventtoOnGridGenerated _output_get (EventDispatchers|CreateEvent :!event OnGridGenerated))
  (EventDispatchers|BindEventtoOnTileDataUpdate _output_get (EventDispatchers|CreateEvent :!event OnTileDataUpdated))
  (bind _returnvalue_2 (Actor|GetActorOfClass "/Game/Blueprints/Core/Combat/BP_CombatSystem.BP_CombatSystem_C"))
  (bind _output_get_2 (Variables|Default|SetCombatSystem _returnvalue_2))
  (EventDispatchers|BindEventtoOnUnitGridIndexChanged _output_get_2 (EventDispatchers|CreateEvent :!event OnUnitGridIndexChanged))
  (EventDispatchers|BindEventtoOnCombatStarted _output_get_2 (EventDispatchers|CreateEvent :!event OnCombatStarted))
  (EventDispatchers|BindEventtoOnCombatEnded _output_get_2 (EventDispatchers|CreateEvent :!event OnCombatEnded))
  (EventDispatchers|BindEventtoOnUnitTurnStarted _output_get_2 (EventDispatchers|CreateEvent :!event OnUNitTurnStarted))
  (EventDispatchers|BindEventtoOnUnitTurnEnded _output_get_2 (EventDispatchers|CreateEvent :!event OnUnitTurnEnded))
  (Input|EnableInput (Game|GetPlayerController 0)))

(event EventTick
  (params (DeltaSeconds :type Float%20%28single-precision%29))
  (CallFunction|UpdateHoveredTileandUnit))

(event Input|MouseEvents|LeftMouseButton
  (params (Key :type Key%20Structure :default "None"))
  (:Pressed
    (CallFunction|UpdateHoveredTileandUnit)
    (Variables|Default|SetIsLeftPressed true)
    (Utilities|IsValid (Variables|Default|GetSelectedActionLeftClick)
      (:Is%20Valid
        (Default|Execute (Variables|Default|GetSelectedActionLeftClick) (Variables|Default|GetHoveredTile)))))
  (:Released
    (Variables|Default|SetIsLeftPressed false)))

(event Input|MouseEvents|RightMouseButton
  (params (Key :type Key%20Structure :default "None"))
  (:Pressed
    (CallFunction|UpdateHoveredTileandUnit)
    (Variables|Default|SetIsRightPressed true)
    (Utilities|IsValid (Variables|Default|GetSelectedActionRightClick)
      (:Is%20Valid
        (Default|Execute (Variables|Default|GetSelectedActionRightClick) (Variables|Default|GetHoveredTile)))))
  (:Released
    (Variables|Default|SetIsRightPressed false)))

(fn ConstructionScript)

(fn UpdateHoveredTileandUnit
  (Utilities|FlowControl|Sequence
    (:then_0
      (bind _unit (CallFunction|GetUnitUnderCursor))
      (if (!= _unit (Variables|Default|GetHoveredUnit))
        (Utilities|FlowControl|Sequence
          (:then_0
            (Utilities|IsValid (Variables|Default|GetHoveredUnit)
              (:Is%20Valid
                (Default|SetHovered (Variables|Default|GetHoveredUnit) false))))
          (:then_1
            (bind _output_get (Variables|Default|SetHoveredUnit _unit))
            (Utilities|IsValid _output_get
              (:Is%20Valid
                (Default|SetHovered _output_get true)))))))
    (:then_1
      (Utilities|IsValid (Variables|Default|GetHoveredUnit)
        (:Is%20Valid
          (LocalVariables|SetNewIndex (Variables|/Game/Blueprints/Core/Units/BP_Unit.BP_Unit_C|GetIndex (Variables|Default|GetHoveredUnit))))
        (:Is%20Not%20Valid
          (bind _index (Default|GetTileIndexUnderCursor (Variables|Default|GetGrid)))
          (LocalVariables|SetNewIndex _index)))
      (if (!= (LocalVariables|GetNewIndex) (Variables|Default|GetHoveredTile))
        (Default|RemoveState (Variables|Default|GetGrid) (Variables|Default|GetHoveredTile) "NewEnumerator1")
        (bind _output_get_2 (Variables|Default|SetHoveredTile (LocalVariables|GetNewIndex)))
        (Default|AddState (Variables|Default|GetGrid) _output_get_2 "NewEnumerator1")
        (CallFunction|OnHoveredTileChanged)))))

(fn SetSelectedActions
  (params (LeftAction :type BP%20Action%20Class%20Reference) (RightAction :type BP%20Action%20Class%20Reference))
  (Utilities|FlowControl|Sequence
    (:then_0
      (Utilities|IsValid (Variables|Default|GetSelectedActionLeftClick)
        (:Is%20Valid
          (Actor|DestroyActor (Variables|Default|GetSelectedActionLeftClick))
          (Variables|Default|SetSelectedActionLeftClick 0))
        (:Is%20Not%20Valid
          _))
      (if (Utilities|IsValidClass LeftAction)
        (bind _returnvalue (Game|SpawnActorfromClass LeftAction (Math|Transform|MakeTransform "0, 0, 0" "0, 0, 0" "1.000000,1.000000,1.000000") "AlwaysSpawn" "MultiplyWithRoot" 0 self 0))
        (Variables|Default|SetSelectedActionLeftClick _returnvalue)))
    (:then_1
      (Utilities|IsValid (Variables|Default|GetSelectedActionRightClick)
        (:Is%20Valid
          (Actor|DestroyActor (Variables|Default|GetSelectedActionRightClick))
          (Variables|Default|SetSelectedActionRightClick 0))
        (:Is%20Not%20Valid
          _))
      (if (Utilities|IsValidClass RightAction)
        (bind _returnvalue_2 (Game|SpawnActorfromClass RightAction (Math|Transform|MakeTransform "0, 0, 0" "0, 0, 0" "1.000000,1.000000,1.000000") "AlwaysSpawn" "MultiplyWithRoot" 0 self 0))
        (Variables|Default|SetSelectedActionRightClick _returnvalue_2)))
    (:then_2
      (Default|CallOnSelectedActionsChanged (Variables|Default|GetSelectedActionLeftClick) (Variables|Default|GetSelectedActionRightClick)))))

(fn GetUnitUnderCursor
  (params (PlayerIndex :type Integer))
  (bind _returnvalue (Game|GetPlayerController PlayerIndex))
  (bind (_hitresult _returnvalue_2) (Game|Player|GetHitResultUnderCursorbyChannel _returnvalue "TraceTypeQuery5" false))
  (if _returnvalue_2
    (return (.AsBP%20Unit (Utilities|Casting|CastToBP_Unit (.HitActor (Collision|BreakHitResult _hitresult)))))
    (else
      (bind _index (Default|GetTileIndexUnderCursor (Variables|Default|GetGrid) PlayerIndex))
      (return (.UnitOnTile (Utilities|Struct|BreakS_TileData (.Value (Utilities|Map|Find (Variables|/Game/Blueprints/Core/Grid/BP_Grid.BP_Grid_C|GetGridTiles (Variables|Default|GetGrid)) _index))))))))

(fn OnGridGenerated
  (if (Default|IsIndexValid (Variables|Default|GetGrid) (Variables|Default|GetSelectedTile))
    (CallFunction|SetSelectedTileandUnit (Variables|Default|GetSelectedTile) true)
    (else
      (CallFunction|SetSelectedTileandUnit (Utilities|Struct|MakeIntPoint -9999 -9999) true))))

(fn OnTileDataUpdated
  (params (Index :type Int%20Point%20Structure))
  (if (Class|KismetMathLibrary|EqualIntPointIntPoint Index (Variables|Default|GetSelectedTile))
    (CallFunction|OnGridGenerated)))

(fn SetSelectedTileandUnit
  (params (Index :type Int%20Point%20Structure) (Force :type Boolean))
  (Utilities|FlowControl|Sequence
    (:then_0
      (if (or (!= Index (Variables|Default|GetSelectedTile)) Force)
        (Default|RemoveState (Variables|Default|GetGrid) (Variables|Default|GetSelectedTile) "NewEnumerator2")
        (Variables|Default|SetSelectedTile Index)
        (Default|AddState (Variables|Default|GetGrid) (Variables|Default|GetSelectedTile) "NewEnumerator2")
        (else
          (Default|RemoveState (Variables|Default|GetGrid) (Variables|Default|GetSelectedTile) "NewEnumerator2")
          (Variables|Default|SetSelectedTile (Utilities|Struct|MakeIntPoint -9999 -9999))))
      (Default|CallOnSelectedTileChanged (Variables|Default|GetSelectedTile)))
    (:then_1
      (LocalVariables|SetNewUnit (.UnitOnTile (Utilities|Struct|BreakS_TileData (.Value (Utilities|Map|Find (Variables|/Game/Blueprints/Core/Grid/BP_Grid.BP_Grid_C|GetGridTiles (Variables|Default|GetGrid)) (Variables|Default|GetSelectedTile))))))
      (if (or (!= (Variables|Default|GetSelectedUnit) (LocalVariables|GetNewUnit)) Force)
        (Utilities|FlowControl|Sequence
          (:then_0
            (Utilities|IsValid (Variables|Default|GetSelectedUnit)
              (:Is%20Valid
                (Default|SetSelected (Variables|Default|GetSelectedUnit) false))))
          (:then_1
            (bind _output_get (Variables|Default|SetSelectedUnit (LocalVariables|GetNewUnit)))
            (Utilities|IsValid _output_get
              (:Is%20Valid
                (Default|SetSelected (LocalVariables|GetNewUnit) true)))))))))

(fn OnUnitGridIndexChanged
  (params (Unit :type BP%20Unit%20Object%20Reference))
  (if (== Unit (Variables|Default|GetSelectedUnit))
    (CallFunction|SetSelectedTileandUnit (Variables|/Game/Blueprints/Core/Units/BP_Unit.BP_Unit_C|GetIndex Unit) false)))

(fn OnCombatStarted
  (CallFunction|SetSelectedActions)
  (CallFunction|SetSelectedTileandUnit (Utilities|Struct|MakeIntPoint -999 -999) false)
  (bind _returnvalue (UserInterface|CreateWidget "/Game/Blueprints/Core/Combat/Widgets/W_Combat.W_Combat_C" 0 self))
  (bind _output_get (Variables|Default|SetWidgetCombat _returnvalue))
  (UserInterface|Viewport|AddtoPlayerScreen _output_get))

(fn OnCombatEnded
  (CallFunction|SetSelectedActions)
  (CallFunction|SetSelectedTileandUnit (Utilities|Struct|MakeIntPoint -999 -999) false)
  (Widget|RemovefromParent (Variables|Default|GetWidgetCombat))
  (Variables|Default|SetWidgetCombat 0))

(fn OnUnitTurnStarted
  (params (Unit :type BP%20Unit%20Object%20Reference))
  (CallFunction|SetSelectedTileandUnit (Variables|/Game/Blueprints/Core/Units/BP_Unit.BP_Unit_C|GetIndex Unit) false))

(fn OnUnitTurnEnded
  (params (Unit :type BP%20Unit%20Object%20Reference))
  (CallFunction|SetSelectedTileandUnit (Utilities|Struct|MakeIntPoint -999 -999) false))