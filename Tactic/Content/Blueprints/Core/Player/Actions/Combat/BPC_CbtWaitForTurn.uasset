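; Player combat action component for the wait-for-turn state that highlights the tiles a unit can reach.
; On hover it targets the hovered unit, falling back to the selected one, and recomputes only when that unit changes.
; Time-sliced grid pathfinding uses the unit's current movement points, valid tile types and diagonal rule.
; The completion callback marks returned tiles with a state, which is cleared on unit change and EndPlay.
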(event EventBeginPlay
  (|CallParentFunction)
  (EventDispatchers|BindEventtoOnPathfindingComplited (Variables|/Game/Blueprints/Core/Grid/BP_Grid.BP_Grid_C|GetPathfindingReachable (Variables|/Game/Blueprints/Core/Player/BP_PlayerActions.BP_PlayerActions_C|GetGrid (Variables|Default|GetPlayerActions))) (EventDispatchers|CreateEvent :!event OnPathfindingCompleatedReachables)))

(event EventEndPlay
  (params (EndPlayReason :type EEndPlayReason%20Enum :default "Destroyed"))
  (|CallParentFunction EndPlayReason)
  (Default|ClearStatesfromTiles (Variables|/Game/Blueprints/Core/Player/BP_PlayerActions.BP_PlayerActions_C|GetGrid (Variables|Default|GetPlayerActions)) "NewEnumerator7"))

(fn ConstructionScript
  (|CallParentFunction))

(fn GenerateReachables
  (params (Unit :type BP%20Unit%20Object%20Reference))
  (if (!= Unit (Variables|Default|GetCurrUnitForReachables))
    (Variables|Default|SetCurrUnitForReachables Unit)
    (Default|ClearStatesfromTiles (Variables|/Game/Blueprints/Core/Player/BP_PlayerActions.BP_PlayerActions_C|GetGrid (Variables|Default|GetPlayerActions)) "NewEnumerator7")
    (Utilities|IsValid (Variables|Default|GetCurrUnitForReachables)
      (:Is%20Valid
        (Default|FindPath (Variables|/Game/Blueprints/Core/Grid/BP_Grid.BP_Grid_C|GetPathfindingReachable (Variables|/Game/Blueprints/Core/Player/BP_PlayerActions.BP_PlayerActions_C|GetGrid (Variables|Default|GetPlayerActions))) (Variables|/Game/Blueprints/Core/Units/BP_Unit.BP_Unit_C|GetIndex (Variables|Default|GetCurrUnitForReachables)) (Utilities|Struct|MakeIntPoint -999 -999) (.CanMoveDiagonaly (Utilities|Struct|BreakS_UnitDataStats (.Stats (Utilities|Struct|BreakS_UnitData (Variables|/Game/Blueprints/Core/Units/BP_Unit.BP_Unit_C|GetUnitData (Variables|Default|GetCurrUnitForReachables)))))) 0.1 15.0 (.ValidTileTypes (Utilities|Struct|BreakS_UnitDataStats (.Stats (Utilities|Struct|BreakS_UnitData (Variables|/Game/Blueprints/Core/Units/BP_Unit.BP_Unit_C|GetUnitData (Variables|Default|GetCurrUnitForReachables)))))) true (.MP_Current (Utilities|Struct|BreakS_UnitDataStats (.Stats (Utilities|Struct|BreakS_UnitData (Variables|/Game/Blueprints/Core/Units/BP_Unit.BP_Unit_C|GetUnitData (Variables|Default|GetCurrUnitForReachables)))))))))))

(fn OnPathfindingCompleatedReachables
  (params (Path :type Array%20of%20Int%20Point%20Structures))
  (for _array_element Path
    (Default|AddState (Variables|/Game/Blueprints/Core/Player/BP_PlayerActions.BP_PlayerActions_C|GetGrid (Variables|Default|GetPlayerActions)) _array_element "NewEnumerator7")))

(fn ExecuteHovered
  (params (Index :type Int%20Point%20Structure))
  (bind _playeractions (Variables|Default|GetPlayerActions))
  (bind _hoveredunit (Variables|/Game/Blueprints/Core/Player/BP_PlayerActions.BP_PlayerActions_C|GetHoveredUnit _playeractions))
  (|CallParentFunction Index)
  (Utilities|IsValid _hoveredunit
    (:Is%20Valid
      (CallFunction|GenerateReachables _hoveredunit))
    (:Is%20Not%20Valid
      (CallFunction|GenerateReachables (Variables|/Game/Blueprints/Core/Player/BP_PlayerActions.BP_PlayerActions_C|GetSelectedUnit _playeractions)))))