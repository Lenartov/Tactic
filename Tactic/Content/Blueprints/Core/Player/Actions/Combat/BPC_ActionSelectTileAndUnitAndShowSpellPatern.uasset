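; Player combat action that extends its parent action, presumably tile and unit selection, to show a spell's range pattern on the grid.
; On Execute it runs the parent logic, then clears one tile state from the grid.
; If the selected tile is valid, it gets the spell range from the CombatSystem using that tile as origin and applies the same state to each returned tile.
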(event EventBeginPlay
  (|CallParentFunction) ; This node is disabled and will not be called.\nDrag off pins to build functionality.
)

(event Collision|EventActorBeginOverlap
  (params (OtherActor :type Actor%20Object%20Reference))
  (|CallParentFunction OtherActor) ; This node is disabled and will not be called.\nDrag off pins to build functionality.
)

(event EventTick
  (params (DeltaSeconds :type Float%20%28single-precision%29))
  (|CallParentFunction DeltaSeconds) ; This node is disabled and will not be called.\nDrag off pins to build functionality.
)

(fn ConstructionScript
  (|CallParentFunction))

(fn Execute
  (params (Index :type Int%20Point%20Structure))
  (|CallParentFunction Index)
  (CallFunction|ShowSpellRangePattern))

(fn ShowSpellRangePattern
  (bind _playeractions (Variables|Default|GetPlayerActions))
  (bind _playeractions_2 (Variables|Default|GetPlayerActions))
  (Default|ClearStatesfromTiles (Variables|/Game/Blueprints/Core/Player/BP_PlayerActions.BP_PlayerActions_C|GetGrid (Variables|Default|GetPlayerActions)) "NewEnumerator8")
  (if (Default|IsIndexValid (Variables|/Game/Blueprints/Core/Player/BP_PlayerActions.BP_PlayerActions_C|GetGrid _playeractions) (Variables|/Game/Blueprints/Core/Player/BP_PlayerActions.BP_PlayerActions_C|GetSelectedTile _playeractions))
    (bind _rangeindexes (Default|GetSpellRange (Variables|/Game/Blueprints/Core/Player/BP_PlayerActions.BP_PlayerActions_C|GetCombatSystem _playeractions_2) (Variables|/Game/Blueprints/Core/Player/BP_PlayerActions.BP_PlayerActions_C|GetSelectedTile _playeractions_2) (Variables|Default|GetCast)))
    (for _array_element _rangeindexes
      (Default|AddState (Variables|/Game/Blueprints/Core/Player/BP_PlayerActions.BP_PlayerActions_C|GetGrid (Variables|Default|GetPlayerActions)) _array_element "NewEnumerator8"))))