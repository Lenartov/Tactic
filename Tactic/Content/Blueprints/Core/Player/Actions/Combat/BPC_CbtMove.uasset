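; Player combat action for grid movement that highlights reachable tiles, previews a path and moves the selected unit.
; Hovering shows the movement range of the hovered unit, or of the selected unit plus its path to the hovered tile.
; Two time-sliced pathfinders, limited by movement points, return results through callbacks that set tile states.
; Execute sends the path to CombatSystem, and walk events pause and refresh the highlights.
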(event EventBeginPlay
  (bind _playeractions (Variables|Default|GetPlayerActions))
  (bind _selectedunit (Variables|/Game/Blueprints/Core/Player/BP_PlayerActions.BP_PlayerActions_C|GetSelectedUnit _playeractions))
  (|CallParentFunction)
  (EventDispatchers|BindEventtoOnPathfindingComplited (Variables|/Game/Blueprints/Core/Grid/BP_Grid.BP_Grid_C|GetPathfindingReachable (Variables|/Game/Blueprints/Core/Player/BP_PlayerActions.BP_PlayerActions_C|GetGrid (Variables|Default|GetPlayerActions))) (EventDispatchers|CreateEvent :!event OnPathfindingCompleatedReachables))
  (EventDispatchers|AssignOnPathfindingComplited (Variables|/Game/Blueprints/Core/Grid/BP_Grid.BP_Grid_C|GetPathfinding (Variables|/Game/Blueprints/Core/Player/BP_PlayerActions.BP_PlayerActions_C|GetGrid (Variables|Default|GetPlayerActions))) (EventDispatchers|CreateEvent :!event OnPathfindingCompleatedPath))
  (EventDispatchers|BindEventtoOnUnitStatedWalking _selectedunit (EventDispatchers|CreateEvent :!event OnUnitStartedWalking))
  (EventDispatchers|BindEventtoOnUnitFinishWalking _selectedunit (EventDispatchers|CreateEvent :!event OnUnitFinishedWalking))
  (CallFunction|GenerateReachables (Variables|/Game/Blueprints/Core/Player/BP_PlayerActions.BP_PlayerActions_C|GetSelectedUnit (Variables|Default|GetPlayerActions))))

(event Collision|EventActorBeginOverlap
  (params (OtherActor :type Actor%20Object%20Reference))
  (|CallParentFunction OtherActor) ; This node is disabled and will not be called.\nDrag off pins to build functionality.
)

(event EventTick
  (params (DeltaSeconds :type Float%20%28single-precision%29))
  (|CallParentFunction DeltaSeconds) ; This node is disabled and will not be called.\nDrag off pins to build functionality.
)

(event EventEndPlay
  (params (EndPlayReason :type EEndPlayReason%20Enum :default "Destroyed"))
  (bind _playeractions (Variables|Default|GetPlayerActions))
  (bind _grid (Variables|/Game/Blueprints/Core/Player/BP_PlayerActions.BP_PlayerActions_C|GetGrid _playeractions))
  (|CallParentFunction EndPlayReason)
  (Default|ClearStatesfromTiles _grid "NewEnumerator7")
  (Default|ClearStatesfromTiles _grid "NewEnumerator4"))

(fn ConstructionScript
  (|CallParentFunction))

(fn GenerateReachables
  (params (Unit :type BP%20Unit%20Object%20Reference))
  (if (!= Unit (Variables|Default|GetCurrUnitForReachables))
    (Variables|Default|SetCurrUnitForReachables Unit)
    (Default|ClearStatesfromTiles (Variables|/Game/Blueprints/Core/Player/BP_PlayerActions.BP_PlayerActions_C|GetGrid (Variables|Default|GetPlayerActions)) "NewEnumerator7")
    (Default|FindPath (Variables|/Game/Blueprints/Core/Grid/BP_Grid.BP_Grid_C|GetPathfindingReachable (Variables|/Game/Blueprints/Core/Player/BP_PlayerActions.BP_PlayerActions_C|GetGrid (Variables|Default|GetPlayerActions))) (Variables|/Game/Blueprints/Core/Units/BP_Unit.BP_Unit_C|GetIndex (Variables|Default|GetCurrUnitForReachables)) (Utilities|Struct|MakeIntPoint -999 -999) (.CanMoveDiagonaly (Utilities|Struct|BreakS_UnitDataStats (.Stats (Utilities|Struct|BreakS_UnitData (Variables|/Game/Blueprints/Core/Units/BP_Unit.BP_Unit_C|GetUnitData (Variables|Default|GetCurrUnitForReachables)))))) 0.1 15.0 (.ValidTileTypes (Utilities|Struct|BreakS_UnitDataStats (.Stats (Utilities|Struct|BreakS_UnitData (Variables|/Game/Blueprints/Core/Units/BP_Unit.BP_Unit_C|GetUnitData (Variables|Default|GetCurrUnitForReachables)))))) true (.MP_Current (Utilities|Struct|BreakS_UnitDataStats (.Stats (Utilities|Struct|BreakS_UnitData (Variables|/Game/Blueprints/Core/Units/BP_Unit.BP_Unit_C|GetUnitData (Variables|Default|GetCurrUnitForReachables)))))))))

(fn OnPathfindingCompleatedReachables
  (params (Path :type Array%20of%20Int%20Point%20Structures))
  (if (not (Variables|Default|GetIsUnitWalking))
    (for _array_element Path
      (Default|AddState (Variables|/Game/Blueprints/Core/Player/BP_PlayerActions.BP_PlayerActions_C|GetGrid (Variables|Default|GetPlayerActions)) _array_element "NewEnumerator7"))))

(fn ExecuteHovered
  (params (Index :type Int%20Point%20Structure))
  (bind _playeractions (Variables|Default|GetPlayerActions))
  (bind _hoveredunit (Variables|/Game/Blueprints/Core/Player/BP_PlayerActions.BP_PlayerActions_C|GetHoveredUnit _playeractions))
  (|CallParentFunction Index)
  (if (not (Variables|Default|GetIsUnitWalking))
    (Utilities|IsValid _hoveredunit
      (:Is%20Valid
        (CallFunction|GenerateReachables _hoveredunit))
      (:Is%20Not%20Valid
        (CallFunction|GenerateReachables (Variables|/Game/Blueprints/Core/Player/BP_PlayerActions.BP_PlayerActions_C|GetSelectedUnit _playeractions))
        (CallFunction|GeneratePath)))))

(fn GeneratePath
  (bind _playeractions (Variables|Default|GetPlayerActions))
  (bind _playeractions_2 (Variables|Default|GetPlayerActions))
  (bind _selectedunit (Variables|/Game/Blueprints/Core/Player/BP_PlayerActions.BP_PlayerActions_C|GetSelectedUnit _playeractions))
  (bind _unitdata (Variables|/Game/Blueprints/Core/Units/BP_Unit.BP_Unit_C|GetUnitData _selectedunit))
  (bind _stats (Utilities|Struct|BreakS_UnitData _unitdata))
  (bind (_validtiletypes _canmovediagonaly _mp_current) (Utilities|Struct|BreakS_UnitDataStats _stats))
  (Default|ClearStatesfromTiles (Variables|/Game/Blueprints/Core/Player/BP_PlayerActions.BP_PlayerActions_C|GetGrid (Variables|Default|GetPlayerActions)) "NewEnumerator4")
  (Utilities|Array|Clear (Variables|Default|GetGeneratedPath))
  (Default|FindPath (Variables|/Game/Blueprints/Core/Grid/BP_Grid.BP_Grid_C|GetPathfinding (Variables|/Game/Blueprints/Core/Player/BP_PlayerActions.BP_PlayerActions_C|GetGrid _playeractions_2)) (Variables|/Game/Blueprints/Core/Units/BP_Unit.BP_Unit_C|GetIndex (Variables|/Game/Blueprints/Core/Player/BP_PlayerActions.BP_PlayerActions_C|GetSelectedUnit _playeractions_2)) (Variables|/Game/Blueprints/Core/Player/BP_PlayerActions.BP_PlayerActions_C|GetHoveredTile _playeractions_2) _canmovediagonaly 0.1 15.0 _validtiletypes false _mp_current))

(fn OnPathfindingCompleatedPath
  (params (Path :type Array%20of%20Int%20Point%20Structures))
  (bind _output_get (Variables|Default|SetGeneratedPath Path))
  (for _array_element _output_get
    (Default|AddState (Variables|/Game/Blueprints/Core/Player/BP_PlayerActions.BP_PlayerActions_C|GetGrid (Variables|Default|GetPlayerActions)) _array_element "NewEnumerator4")))

(fn Execute
  (params (Index :type Int%20Point%20Structure))
  (bind _playeractions (Variables|Default|GetPlayerActions))
  (bind _generatedpath (Variables|Default|GetGeneratedPath))
  (|CallParentFunction Index)
  (if (> (Utilities|Array|Length (Variables|Default|GetGeneratedPath)) 0)
    (Default|MoveUnit (Variables|/Game/Blueprints/Core/Player/BP_PlayerActions.BP_PlayerActions_C|GetCombatSystem _playeractions) (Variables|/Game/Blueprints/Core/Player/BP_PlayerActions.BP_PlayerActions_C|GetSelectedUnit _playeractions) _generatedpath 0.25)
    (Utilities|Array|Clear _generatedpath)))

(fn OnUnitStartedWalking
  (params (Unit :type BP%20Unit%20Object%20Reference))
  (Variables|Default|SetIsUnitWalking true)
  (Default|ClearStatesfromTiles (Variables|/Game/Blueprints/Core/Player/BP_PlayerActions.BP_PlayerActions_C|GetGrid (Variables|Default|GetPlayerActions)) "NewEnumerator7")
  (Variables|Default|SetCurrUnitForReachables 0))

(fn OnUnitFinishedWalking
  (params (Unit :type BP%20Unit%20Object%20Reference))
  (Variables|Default|SetIsUnitWalking false)
  (CallFunction|ExecuteHovered (Variables|/Game/Blueprints/Core/Player/BP_PlayerActions.BP_PlayerActions_C|GetHoveredTile (Variables|Default|GetPlayerActions))))