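; Player combat action that casts the selected spell from the selected grid tile onto a target tile.
; Setting a spell loads its cast and area data and marks its range as grid tile states.
; Hovering a tile inside that range marks the area of effect, or just that tile if there is no pattern.
; Execution calls the combat system and resets the spell list selection; clearing the spell or ending play removes both highlights.
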(event EventBeginPlay
  (|CallParentFunction) ; This node is disabled and will not be called.\nDrag off pins to build functionality.
)

(event Collision|EventActorBeginOverlap
  (params (OtherActor :type Actor%20Object%20Reference))
  (|CallParentFunction OtherActor) ; This node is disabled and will not be called.\nDrag off pins to build functionality.
)

(event EventTick
  (params (DeltaSeconds :type Float%20%28single-precision%29))
  (|CallParentFunction DeltaSeconds) ; This node is disabled and will not be called.\nDrag off pins to build functionality.
)

(event EventEndPlay
  (params (EndPlayReason :type EEndPlayReason%20Enum :default "Destroyed"))
  (bind _playeractions (Variables|Default|GetPlayerActions))
  (bind _grid (Variables|/Game/Blueprints/Core/Player/BP_PlayerActions.BP_PlayerActions_C|GetGrid _playeractions))
  (|CallParentFunction EndPlayReason)
  (Default|ClearStatesfromTiles _grid "NewEnumerator8")
  (Default|ClearStatesfromTiles _grid "NewEnumerator9"))

(fn ConstructionScript
  (|CallParentFunction))

(fn SetSpell
  (params (Spell :type E_Spell%20Enum :default "NewEnumerator0"))
  (bind _playeractions (Variables|Default|GetPlayerActions))
  (bind _grid (Variables|/Game/Blueprints/Core/Player/BP_PlayerActions.BP_PlayerActions_C|GetGrid _playeractions))
  (bind _output_get (Variables|Default|SetSpell Spell))
  (if (Utilities|Enum|NotEqual(Enum) _output_get "NewEnumerator0")
    (bind _data (CallFunction|GetSpellDatafromSpell (Variables|Default|GetSpell)))
    (Variables|Default|SetCast (.Cast (Utilities|Struct|BreakS_SpellData _data)))
    (Variables|Default|SetCast%20AOE (.CastAOE (Utilities|Struct|BreakS_SpellData _data)))
    (CallFunction|ShowSpellRangePattern)
    (else
      (Default|ClearStatesfromTiles _grid "NewEnumerator8")
      (Default|ClearStatesfromTiles _grid "NewEnumerator9"))))

(fn ShowSpellRangePattern
  (bind _playeractions (Variables|Default|GetPlayerActions))
  (Utilities|FlowControl|Sequence
    (:then_0
      (Default|ClearStatesfromTiles (Variables|/Game/Blueprints/Core/Player/BP_PlayerActions.BP_PlayerActions_C|GetGrid (Variables|Default|GetPlayerActions)) "NewEnumerator8")
      (bind _rangeindexes (Default|GetSpellRange (Variables|/Game/Blueprints/Core/Player/BP_PlayerActions.BP_PlayerActions_C|GetCombatSystem _playeractions) (Variables|/Game/Blueprints/Core/Player/BP_PlayerActions.BP_PlayerActions_C|GetSelectedTile _playeractions) (Variables|Default|GetCast)))
      (for _array_element _rangeindexes
        (Default|AddState (Variables|/Game/Blueprints/Core/Player/BP_PlayerActions.BP_PlayerActions_C|GetGrid (Variables|Default|GetPlayerActions)) _array_element "NewEnumerator8")))
    (:then_1
      (CallFunction|ShowSpellRangePatternAOE))))

(fn Execute
  (params (Index :type Int%20Point%20Structure))
  (bind _playeractions (Variables|Default|GetPlayerActions))
  (bind _playeractions_2 (Variables|Default|GetPlayerActions))
  (bind _widgetcombat (Variables|/Game/Blueprints/Core/Player/BP_PlayerActions.BP_PlayerActions_C|GetWidgetCombat _playeractions))
  (|CallParentFunction Index)
  (Default|CastSpell (Variables|/Game/Blueprints/Core/Player/BP_PlayerActions.BP_PlayerActions_C|GetCombatSystem _playeractions_2) (Variables|Default|GetSpell) (Variables|/Game/Blueprints/Core/Player/BP_PlayerActions.BP_PlayerActions_C|GetSelectedTile _playeractions_2) Index)
  (Utilities|IsValid _widgetcombat
    (:Is%20Valid
      (Default|SetSelectedSpellfromIndex (Variables|/Game/Blueprints/Core/Combat/Widgets/W_Combat.W_Combat_C|GetButton_ListSpells _widgetcombat) -1))))

(fn ShowSpellRangePatternAOE
  (bind _playeractions (Variables|Default|GetPlayerActions))
  (bind _playeractions_2 (Variables|Default|GetPlayerActions))
  (Default|ClearStatesfromTiles (Variables|/Game/Blueprints/Core/Player/BP_PlayerActions.BP_PlayerActions_C|GetGrid (Variables|Default|GetPlayerActions)) "NewEnumerator9")
  (if (Utilities|Array|ContainsItem (Utilities|Struct|BreakS_IntPointArray (.Value (Utilities|Map|Find (Variables|/Game/Blueprints/Core/Grid/BP_Grid.BP_Grid_C|GetTileStatesToIndexes (Variables|/Game/Blueprints/Core/Player/BP_PlayerActions.BP_PlayerActions_C|GetGrid (Variables|Default|GetPlayerActions))) "NewEnumerator8"))) (Variables|/Game/Blueprints/Core/Player/BP_PlayerActions.BP_PlayerActions_C|GetHoveredTile (Variables|Default|GetPlayerActions)))
    (if (Utilities|Enum|NotEqual(Enum) (.RangePatern (Utilities|Struct|BreakS_SpellDataCast (Variables|Default|GetCast%20AOE))) "NewEnumerator0")
      (bind _rangeindexes (Default|GetSpellRange (Variables|/Game/Blueprints/Core/Player/BP_PlayerActions.BP_PlayerActions_C|GetCombatSystem _playeractions) (Variables|/Game/Blueprints/Core/Player/BP_PlayerActions.BP_PlayerActions_C|GetHoveredTile _playeractions) (Variables|Default|GetCast%20AOE)))
      (for _array_element _rangeindexes
        (Default|AddState (Variables|/Game/Blueprints/Core/Player/BP_PlayerActions.BP_PlayerActions_C|GetGrid (Variables|Default|GetPlayerActions)) _array_element "NewEnumerator9"))
      (else
        (Default|AddState (Variables|/Game/Blueprints/Core/Player/BP_PlayerActions.BP_PlayerActions_C|GetGrid _playeractions_2) (Variables|/Game/Blueprints/Core/Player/BP_PlayerActions.BP_PlayerActions_C|GetHoveredTile _playeractions_2) "NewEnumerator9")))))

(fn ExecuteHovered
  (params (Index :type Int%20Point%20Structure))
  (|CallParentFunction Index)
  (CallFunction|ShowSpellRangePatternAOE))