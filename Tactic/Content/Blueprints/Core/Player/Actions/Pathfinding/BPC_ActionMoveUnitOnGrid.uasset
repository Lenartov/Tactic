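; Player action that moves the selected unit across the grid to a target tile index.
; Execute clears path highlights, then requests a path using the unit's diagonal rule, valid tile types and current movement points.
; The pathfinding-complete callback highlights the path, hands it to the combat system for movement and calls ResetMP.
; Highlights clear when the unit finishes walking; EndPlay also runs Execute with a sentinel index.
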(event EventBeginPlay
  (|CallParentFunction) ; This node is disabled and will not be called.\nDrag off pins to build functionality.
)

(event Collision|EventActorBeginOverlap
  (params (OtherActor :type Actor%20Object%20Reference))
  (|CallParentFunction OtherActor) ; This node is disabled and will not be called.\nDrag off pins to build functionality.
)

(event EventTick
  (params (DeltaSeconds :type Float%20%28single-precision%29))
  (|CallParentFunction DeltaSeconds) ; This node is disabled and will not be called.\nDrag off pins to build functionality.
)

(event EventEndPlay
  (params (EndPlayReason :type EEndPlayReason%20Enum :default "Destroyed"))
  (CallFunction|Execute (Utilities|Struct|MakeIntPoint -9999 -9999)))

(fn ConstructionScript
  (|CallParentFunction))

(fn Execute
  (params (Index :type Int%20Point%20Structure))
  (Default|ClearStatesfromTiles (Variables|/Game/Blueprints/Core/Player/BP_PlayerActions.BP_PlayerActions_C|GetGrid (Variables|Default|GetPlayerActions)) "NewEnumerator4")
  (bind _output_get (Variables|Default|SetCurrentUnit (Variables|/Game/Blueprints/Core/Player/BP_PlayerActions.BP_PlayerActions_C|GetSelectedUnit (Variables|Default|GetPlayerActions))))
  (Utilities|IsValid _output_get
    (:Is%20Valid
      (EventDispatchers|BindEventtoOnUnitFinishWalking (Variables|Default|GetCurrentUnit) (EventDispatchers|CreateEvent :!event OnUnitFinishedWalking))
      (EventDispatchers|BindEventtoOnPathfindingComplited (Variables|/Game/Blueprints/Core/Grid/BP_Grid.BP_Grid_C|GetPathfinding (Variables|/Game/Blueprints/Core/Player/BP_PlayerActions.BP_PlayerActions_C|GetGrid (Variables|Default|GetPlayerActions))) (EventDispatchers|CreateEvent :!event OnPathfindingComplited))
      (Default|FindPath (Variables|/Game/Blueprints/Core/Grid/BP_Grid.BP_Grid_C|GetPathfinding (Variables|/Game/Blueprints/Core/Player/BP_PlayerActions.BP_PlayerActions_C|GetGrid (Variables|Default|GetPlayerActions))) (Variables|/Game/Blueprints/Core/Player/BP_PlayerActions.BP_PlayerActions_C|GetSelectedTile (Variables|Default|GetPlayerActions)) Index (.CanMoveDiagonaly (Utilities|Struct|BreakS_UnitDataStats (.Stats (Utilities|Struct|BreakS_UnitData (Variables|/Game/Blueprints/Core/Units/BP_Unit.BP_Unit_C|GetUnitData (Variables|Default|GetCurrentUnit)))))) 0.0 0.0 (.ValidTileTypes (Utilities|Struct|BreakS_UnitDataStats (.Stats (Utilities|Struct|BreakS_UnitData (Variables|/Game/Blueprints/Core/Units/BP_Unit.BP_Unit_C|GetUnitData (Variables|Default|GetCurrentUnit)))))) false (.MP_Current (Utilities|Struct|BreakS_UnitDataStats (.Stats (Utilities|Struct|BreakS_UnitData (Variables|/Game/Blueprints/Core/Units/BP_Unit.BP_Unit_C|GetUnitData (Variables|Default|GetCurrentUnit))))))))))

(fn OnPathfindingComplited
  (params (Path :type Array%20of%20Int%20Point%20Structures))
  (bind _currentunit (Variables|Default|GetCurrentUnit))
  (Utilities|IsValid (Variables|Default|GetCurrentUnit)
    (:Is%20Valid
      (if (== (Variables|Default|GetCurrentUnit) (Variables|/Game/Blueprints/Core/Player/BP_PlayerActions.BP_PlayerActions_C|GetSelectedUnit (Variables|Default|GetPlayerActions)))
        (for _array_element Path
          (Default|AddState (Variables|/Game/Blueprints/Core/Player/BP_PlayerActions.BP_PlayerActions_C|GetGrid (Variables|Default|GetPlayerActions)) _array_element "NewEnumerator4"))
        (Default|MoveUnit (Variables|/Game/Blueprints/Core/Player/BP_PlayerActions.BP_PlayerActions_C|GetCombatSystem (Variables|Default|GetPlayerActions)) _currentunit Path (Variables|Default|GetMove%20Duration%20Per%20Tile))
        (Default|ResetMP _currentunit)))))

(fn OnUnitFinishedWalking
  (params (Unit :type BP%20Unit%20Object%20Reference))
  (if (== Unit (Variables|Default|GetCurrentUnit))
    (Default|ClearStatesfromTiles (Variables|/Game/Blueprints/Core/Player/BP_PlayerActions.BP_PlayerActions_C|GetGrid (Variables|Default|GetPlayerActions)) "NewEnumerator4")))