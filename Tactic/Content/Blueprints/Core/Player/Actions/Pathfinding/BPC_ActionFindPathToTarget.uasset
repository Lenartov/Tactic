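; Player action that finds a path from the selected grid tile to a target tile and marks it with a tile state.
; Execute clears that state, then calls the grid's Pathfinding with diagonal, flying, max length and iteration timing options.
; The completion callback adds the state to each path tile.
; Selection changes and EndPlay re-run Execute with an out-of-range target, clearing the shown path.
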(event Custom|OnSelectedTileChanged
  (params (Index :type Int%20Point%20Structure))
  (CallFunction|Execute (Utilities|Struct|MakeIntPoint -999 -999)))

(event EventBeginPlay
  (|CallParentFunction)
  (EventDispatchers|BindEventtoOnSelectedTileChanged (Variables|Default|GetPlayerActions) (delegate Custom|OnSelectedTileChanged)))

(event EventEndPlay
  (params (EndPlayReason :type EEndPlayReason%20Enum :default "Destroyed"))
  (CallFunction|Execute (Utilities|Struct|MakeIntPoint -9999 -9999)))

(fn ConstructionScript
  (|CallParentFunction))

(fn Execute
  (params (Index :type Int%20Point%20Structure))
  (Default|ClearStatesfromTiles (Variables|/Game/Blueprints/Core/Player/BP_PlayerActions.BP_PlayerActions_C|GetGrid (Variables|Default|GetPlayerActions)) "NewEnumerator4")
  (EventDispatchers|BindEventtoOnPathfindingComplited (Variables|/Game/Blueprints/Core/Grid/BP_Grid.BP_Grid_C|GetPathfinding (Variables|/Game/Blueprints/Core/Player/BP_PlayerActions.BP_PlayerActions_C|GetGrid (Variables|Default|GetPlayerActions))) (EventDispatchers|CreateEvent :!event OnPathfindingComplited))
  (Default|FindPath (Variables|/Game/Blueprints/Core/Grid/BP_Grid.BP_Grid_C|GetPathfinding (Variables|/Game/Blueprints/Core/Player/BP_PlayerActions.BP_PlayerActions_C|GetGrid (Variables|Default|GetPlayerActions))) (Variables|/Game/Blueprints/Core/Player/BP_PlayerActions.BP_PlayerActions_C|GetSelectedTile (Variables|Default|GetPlayerActions)) Index (Variables|Default|GetIncludeDiagonals) (Variables|Default|GetDelay%20Iteration) (Variables|Default|GetMax%20Ms%20Per%20Frame) (select (Variables|Default|GetIncludeFlying) (Utilities|Array|MakeArray "NewEnumerator1" "NewEnumerator3" "NewEnumerator4" "NewEnumerator5") (Utilities|Array|MakeArray "NewEnumerator1" "NewEnumerator3" "NewEnumerator4")) false (Variables|Default|GetMaxLength)))

(fn OnPathfindingComplited
  (params (Path :type Array%20of%20Int%20Point%20Structures))
  (for _array_element Path
    (Default|AddState (Variables|/Game/Blueprints/Core/Player/BP_PlayerActions.BP_PlayerActions_C|GetGrid (Variables|Default|GetPlayerActions)) _array_element "NewEnumerator4")))