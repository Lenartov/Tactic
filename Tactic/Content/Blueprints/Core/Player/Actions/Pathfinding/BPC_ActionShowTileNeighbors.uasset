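; Player action that highlights the valid neighbors of a given grid tile, apparently as a visual check on pathfinding.
; Execute clears the neighbor state from the grid, asks the grid's Pathfinding for neighbors filtered by allowed tile types and optional diagonals, then adds that state to each result.
; EndPlay reruns Execute with an out-of-range index to clear the highlights when the action is removed.
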(event EventBeginPlay
  (|CallParentFunction) ; This node is disabled and will not be called.\nDrag off pins to build functionality.
)

(event Collision|EventActorBeginOverlap
  (params (OtherActor :type Actor%20Object%20Reference))
  (|CallParentFunction OtherActor) ; This node is disabled and will not be called.\nDrag off pins to build functionality.
)

(event EventTick
  (params (DeltaSeconds :type Float%20%28single-precision%29))
  (|CallParentFunction DeltaSeconds) ; This node is disabled and will not be called.\nDrag off pins to build functionality.
)

(event EventEndPlay
  (params (EndPlayReason :type EEndPlayReason%20Enum :default "Destroyed"))
  (CallFunction|Execute (Utilities|Struct|MakeIntPoint -9999 -9999)))

(fn ConstructionScript
  (|CallParentFunction))

(fn Execute
  (params (Index :type Int%20Point%20Structure))
  (Default|ClearStatesfromTiles (Variables|/Game/Blueprints/Core/Player/BP_PlayerActions.BP_PlayerActions_C|GetGrid (Variables|Default|GetPlayerActions)) "NewEnumerator3")
  (bind _neighbor (Default|GetValidTileNeighbor (Variables|/Game/Blueprints/Core/Grid/BP_Grid.BP_Grid_C|GetPathfinding (Variables|/Game/Blueprints/Core/Player/BP_PlayerActions.BP_PlayerActions_C|GetGrid (Variables|Default|GetPlayerActions))) Index (Variables|Default|GetIncludeDiagonals) (Utilities|Array|MakeArray "NewEnumerator1" "NewEnumerator3" "NewEnumerator4" "NewEnumerator5")))
  (for _array_element _neighbor
    (Default|AddState (Variables|/Game/Blueprints/Core/Player/BP_PlayerActions.BP_PlayerActions_C|GetGrid (Variables|Default|GetPlayerActions)) (.index _array_element) "NewEnumerator3")))