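; Player action component that adds a tile to the grid at a given index.
; Execute runs only when the index is not already valid in the grid.
; It ground-traces from the index's location, then adds a tile of a fixed type at that point, using the grid's rotation for the index and its tile scale.
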(fn ConstructionScript
  (|CallParentFunction))

(fn Execute
  (params (Index :type Int%20Point%20Structure))
  (bind _playeractions (Variables|Default|GetPlayerActions))
  (bind _playeractions_2 (Variables|Default|GetPlayerActions))
  (bind _grid (Variables|/Game/Blueprints/Core/Player/BP_PlayerActions.BP_PlayerActions_C|GetGrid _playeractions))
  (bind _grid_2 (Variables|/Game/Blueprints/Core/Player/BP_PlayerActions.BP_PlayerActions_C|GetGrid _playeractions_2))
  (if (not (Default|IsIndexValid (Variables|/Game/Blueprints/Core/Player/BP_PlayerActions.BP_PlayerActions_C|GetGrid (Variables|Default|GetPlayerActions)) Index))
    (bind _outlocation (Default|TraceforGround _grid_2 (Default|GetLocationfromIndex _grid Index)))
    (Default|AddGridTile _grid_2 (Utilities|Struct|MakeS_TileData Index "NewEnumerator1" (Math|Transform|MakeTransform _outlocation (Default|GetRotationfromIndex _grid Index) (Default|GetTileScale _grid)) "NewEnumerator0" 0))))