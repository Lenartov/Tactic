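; Player grid action that extends its parent's Execute, presumably tile and unit selection, to mark the tiles reachable from the selected tile.
; GenerateReachable clears old marks and runs the grid's reachable pathfinder using the selected unit's movement stats, or configurable search settings without a unit.
; A completion callback adds the tile state to each result.
; Unit walk events clear the marks on start and regenerate them on finish.
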(event EventBeginPlay
  (|CallParentFunction) ; This node is disabled and will not be called.\nDrag off pins to build functionality.
)

(event Collision|EventActorBeginOverlap
  (params (OtherActor :type Actor%20Object%20Reference))
  (|CallParentFunction OtherActor) ; This node is disabled and will not be called.\nDrag off pins to build functionality.
)

(event EventTick
  (params (DeltaSeconds :type Float%20%28single-precision%29))
  (|CallParentFunction DeltaSeconds) ; This node is disabled and will not be called.\nDrag off pins to build functionality.
)

(fn ConstructionScript
  (|CallParentFunction))

(fn GenerateReachable
  (bind _playeractions (Variables|Default|GetPlayerActions))
  (bind _playeractions_2 (Variables|Default|GetPlayerActions))
  (bind _selectedunit (Variables|/Game/Blueprints/Core/Player/BP_PlayerActions.BP_PlayerActions_C|GetSelectedUnit _playeractions))
  (bind _selectedunit_2 (Variables|/Game/Blueprints/Core/Player/BP_PlayerActions.BP_PlayerActions_C|GetSelectedUnit _playeractions_2))
  (bind _unitdata (Variables|/Game/Blueprints/Core/Units/BP_Unit.BP_Unit_C|GetUnitData _selectedunit))
  (bind _stats (Utilities|Struct|BreakS_UnitData _unitdata))
  (bind (_validtiletypes _canmovediagonaly _mp_current) (Utilities|Struct|BreakS_UnitDataStats _stats))
  (Default|ClearStatesfromTiles (Variables|/Game/Blueprints/Core/Player/BP_PlayerActions.BP_PlayerActions_C|GetGrid (Variables|Default|GetPlayerActions)) "NewEnumerator7")
  (EventDispatchers|BindEventtoOnPathfindingComplited (Variables|/Game/Blueprints/Core/Grid/BP_Grid.BP_Grid_C|GetPathfindingReachable (Variables|/Game/Blueprints/Core/Player/BP_PlayerActions.BP_PlayerActions_C|GetGrid (Variables|Default|GetPlayerActions))) (EventDispatchers|CreateEvent :!event OnPathfindingCompleated))
  (Utilities|IsValid (Variables|/Game/Blueprints/Core/Player/BP_PlayerActions.BP_PlayerActions_C|GetSelectedUnit (Variables|Default|GetPlayerActions))
    (:Is%20Valid
      (EventDispatchers|BindEventtoOnUnitStatedWalking _selectedunit_2 (EventDispatchers|CreateEvent :!event OnStartedWalking))
      (EventDispatchers|BindEventtoOnUnitFinishWalking _selectedunit_2 (EventDispatchers|CreateEvent :!event OnFinishWalking))
      (Default|FindPath :self (Variables|/Game/Blueprints/Core/Grid/BP_Grid.BP_Grid_C|GetPathfindingReachable (Variables|/Game/Blueprints/Core/Player/BP_PlayerActions.BP_PlayerActions_C|GetGrid (Variables|Default|GetPlayerActions))) :Start (Variables|/Game/Blueprints/Core/Player/BP_PlayerActions.BP_PlayerActions_C|GetSelectedTile (Variables|Default|GetPlayerActions)) :Diagonals _canmovediagonaly :Valid%20Types _validtiletypes :ReturnReachable true :Length _mp_current))
    (:Is%20Not%20Valid
      (Default|FindPath (Variables|/Game/Blueprints/Core/Grid/BP_Grid.BP_Grid_C|GetPathfindingReachable (Variables|/Game/Blueprints/Core/Player/BP_PlayerActions.BP_PlayerActions_C|GetGrid (Variables|Default|GetPlayerActions))) (Variables|/Game/Blueprints/Core/Player/BP_PlayerActions.BP_PlayerActions_C|GetSelectedTile (Variables|Default|GetPlayerActions)) (Utilities|Struct|MakeIntPoint -999 -999) (Variables|Default|GetIncludeDiagonals) (Variables|Default|GetDelayBetweenIterations) (Variables|Default|GetMaxMsPerFrame) (select (Variables|Default|GetIncludeFlying) (Utilities|Array|MakeArray "NewEnumerator1" "NewEnumerator3" "NewEnumerator4" "NewEnumerator5") (Utilities|Array|MakeArray "NewEnumerator1" "NewEnumerator3" "NewEnumerator4")) true (Variables|Default|GetMaxPathLenght)))))

(fn Execute
  (params (Index :type Int%20Point%20Structure))
  (|CallParentFunction Index)
  (CallFunction|GenerateReachable))

(fn OnPathfindingCompleated
  (params (Path :type Array%20of%20Int%20Point%20Structures))
  (for _array_element Path
    (Default|AddState (Variables|/Game/Blueprints/Core/Player/BP_PlayerActions.BP_PlayerActions_C|GetGrid (Variables|Default|GetPlayerActions)) _array_element "NewEnumerator7")))

(fn OnStartedWalking
  (params (Unit :type BP%20Unit%20Object%20Reference))
  (Default|ClearStatesfromTiles (Variables|/Game/Blueprints/Core/Player/BP_PlayerActions.BP_PlayerActions_C|GetGrid (Variables|Default|GetPlayerActions)) "NewEnumerator7"))

(fn OnFinishWalking
  (params (Unit :type BP%20Unit%20Object%20Reference))
  (CallFunction|GenerateReachable))