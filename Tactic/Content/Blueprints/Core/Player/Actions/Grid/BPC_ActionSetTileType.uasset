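; Player action component that changes the type of a grid tile at a given index.
; Execute checks that the index is valid on the player actions' grid, then looks up that tile's existing data.
; It re-adds the tile with the action's TileType while keeping its index, transform, states and unit on the tile.
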(fn ConstructionScript
  (|CallParentFunction))

(fn Execute
  (params (Index :type Int%20Point%20Structure))
  (if (Default|IsIndexValid (Variables|/Game/Blueprints/Core/Player/BP_PlayerActions.BP_PlayerActions_C|GetGrid (Variables|Default|GetPlayerActions)) Index)
    (LocalVariables|SetData (.Value (Utilities|Map|Find (Variables|/Game/Blueprints/Core/Grid/BP_Grid.BP_Grid_C|GetGridTiles (Variables|/Game/Blueprints/Core/Player/BP_PlayerActions.BP_PlayerActions_C|GetGrid (Variables|Default|GetPlayerActions))) Index)))
    (Default|AddGridTile (Variables|/Game/Blueprints/Core/Player/BP_PlayerActions.BP_PlayerActions_C|GetGrid (Variables|Default|GetPlayerActions)) (Utilities|Struct|MakeS_TileData (.index (LocalVariables|GetData)) (Variables|Default|GetTileType) (.transform (LocalVariables|GetData)) (.states (LocalVariables|GetData)) (.unitontile (LocalVariables|GetData))))))