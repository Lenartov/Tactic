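; Player grid action that raises or lowers the tile at a given index.
; Execute checks that the index is valid, then reads that tile's data from the GridTiles map on the player's Grid.
; It re-adds the tile through AddGridTile with its location moved one tile-size Z step up or down, chosen by IsIncrease, keeping all other data unchanged.
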(fn ConstructionScript
  (|CallParentFunction))

(fn Execute
  (params (Index :type Int%20Point%20Structure))
  (if (Default|IsIndexValid (Variables|/Game/Blueprints/Core/Player/BP_PlayerActions.BP_PlayerActions_C|GetGrid (Variables|Default|GetPlayerActions)) Index)
    (LocalVariables|SetData (.Value (Utilities|Map|Find (Variables|/Game/Blueprints/Core/Grid/BP_Grid.BP_Grid_C|GetGridTiles (Variables|/Game/Blueprints/Core/Player/BP_PlayerActions.BP_PlayerActions_C|GetGrid (Variables|Default|GetPlayerActions))) Index)))
    (Default|AddGridTile (Variables|/Game/Blueprints/Core/Player/BP_PlayerActions.BP_PlayerActions_C|GetGrid (Variables|Default|GetPlayerActions)) (Utilities|Struct|MakeS_TileData (.index (LocalVariables|GetData)) (.tiletype (LocalVariables|GetData)) (Math|Transform|MakeTransform (+ (.Location (Math|Transform|BreakTransform (.transform (LocalVariables|GetData)))) (Math|Vector|MakeVector 0.0 0.0 (* (.z (Variables|/Game/Blueprints/Core/Grid/BP_Grid.BP_Grid_C|GetTile%20Size (Variables|/Game/Blueprints/Core/Player/BP_PlayerActions.BP_PlayerActions_C|GetGrid (Variables|Default|GetPlayerActions)))) (Math|Float|SelectFloat 1.0 -1.0 (Variables|Default|GetIsIncrease))))) (.Rotation (Math|Transform|BreakTransform (.transform (LocalVariables|GetData)))) (.Scale (Math|Transform|BreakTransform (.transform (LocalVariables|GetData))))) (.states (LocalVariables|GetData)) (.unitontile (LocalVariables|GetData))))))