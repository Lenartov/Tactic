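; Player grid action that fills pathfinding data with each tile's minimum cost to the selected tile.
; On Execute it runs the parent action, clears previously generated pathfinding data and checks that the selected tile is valid.
; It then registers every grid tile as discovered with zero cost from start and that heuristic cost, optionally counting diagonals, without running a path search.
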(event EventBeginPlay
  (|CallParentFunction) ; This node is disabled and will not be called.\nDrag off pins to build functionality.
)

(event Collision|EventActorBeginOverlap
  (params (OtherActor :type Actor%20Object%20Reference))
  (|CallParentFunction OtherActor) ; This node is disabled and will not be called.\nDrag off pins to build functionality.
)

(event EventTick
  (params (DeltaSeconds :type Float%20%28single-precision%29))
  (|CallParentFunction DeltaSeconds) ; This node is disabled and will not be called.\nDrag off pins to build functionality.
)

(fn ConstructionScript
  (|CallParentFunction))

(fn Execute
  (params (Index :type Int%20Point%20Structure))
  (bind _playeractions (Variables|Default|GetPlayerActions))
  (bind _playeractions_2 (Variables|Default|GetPlayerActions))
  (bind _grid (Variables|/Game/Blueprints/Core/Player/BP_PlayerActions.BP_PlayerActions_C|GetGrid _playeractions))
  (bind _grid_2 (Variables|/Game/Blueprints/Core/Player/BP_PlayerActions.BP_PlayerActions_C|GetGrid _playeractions_2))
  (|CallParentFunction Index)
  (Default|ClearGeneratedData (Variables|/Game/Blueprints/Core/Grid/BP_Grid.BP_Grid_C|GetPathfinding _grid))
  (if (Default|IsIndexValid _grid (Variables|/Game/Blueprints/Core/Player/BP_PlayerActions.BP_PlayerActions_C|GetSelectedTile _playeractions))
    (bind _keys (Utilities|Map|Keys (Variables|/Game/Blueprints/Core/Grid/BP_Grid.BP_Grid_C|GetGridTiles _grid_2)))
    (for _array_element _keys
      (Default|DiscoverTile (Variables|/Game/Blueprints/Core/Grid/BP_Grid.BP_Grid_C|GetPathfinding (Variables|/Game/Blueprints/Core/Player/BP_PlayerActions.BP_PlayerActions_C|GetGrid (Variables|Default|GetPlayerActions))) (Utilities|Struct|MakeS_PathfindingData _array_element 1 0 (Default|GetMinCostBetweenTiles (Variables|/Game/Blueprints/Core/Grid/BP_Grid.BP_Grid_C|GetPathfinding _grid_2) _array_element (Variables|/Game/Blueprints/Core/Player/BP_PlayerActions.BP_PlayerActions_C|GetSelectedTile _playeractions_2) (Variables|Default|GetIncludeDiagonal)) "(X=-9999,Y=-9999)")))))