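; Player action for combat setup that adds or removes a unit on the grid tile at a given index.
; When adding, it checks that the tile type is valid for the chosen unit type, clears any occupant, then spawns a BP_Unit and registers it with the combat system by team and AI flag.
; When removing, it reuses the clearing step, which takes the unit out of combat and destroys it.
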(event EventBeginPlay
  (|CallParentFunction) ; This node is disabled and will not be called.\nDrag off pins to build functionality.
)

(event Collision|EventActorBeginOverlap
  (params (OtherActor :type Actor%20Object%20Reference))
  (|CallParentFunction OtherActor) ; This node is disabled and will not be called.\nDrag off pins to build functionality.
)

(event EventTick
  (params (DeltaSeconds :type Float%20%28single-precision%29))
  (|CallParentFunction DeltaSeconds) ; This node is disabled and will not be called.\nDrag off pins to build functionality.
)

(fn ConstructionScript
  (|CallParentFunction))

(fn Execute
  (params (Index :type Int%20Point%20Structure))
  (bind _playeractions (Variables|Default|GetPlayerActions))
  (bind _grid (Variables|/Game/Blueprints/Core/Player/BP_PlayerActions.BP_PlayerActions_C|GetGrid _playeractions))
  (bind _gridtiles (Variables|/Game/Blueprints/Core/Grid/BP_Grid.BP_Grid_C|GetGridTiles _grid))
  (bind _value (Utilities|Map|Find _gridtiles Index))
  (bind _unitontile (Utilities|Struct|BreakS_TileData _value))
  (if (Variables|Default|GetIsAddingUnit)
    (bind _data (CallFunction|GetDefaultUnitDatafromType (Variables|Default|GetUnitType)))
    (if (Utilities|Array|ContainsItem (.ValidTileTypes (Utilities|Struct|BreakS_UnitDataStats (.Stats (Utilities|Struct|BreakS_UnitData _data)))) (.TileType (Utilities|Struct|BreakS_TileData (.Value (Utilities|Map|Find (Variables|/Game/Blueprints/Core/Grid/BP_Grid.BP_Grid_C|GetGridTiles (Variables|/Game/Blueprints/Core/Player/BP_PlayerActions.BP_PlayerActions_C|GetGrid (Variables|Default|GetPlayerActions))) Index)))))
      (Utilities|FlowControl|Sequence
        (:then_0
          (Utilities|IsValid _unitontile :!label _label
            (:Is%20Valid
              (Default|RemoveUnitfromCombat (Variables|/Game/Blueprints/Core/Player/BP_PlayerActions.BP_PlayerActions_C|GetCombatSystem (Variables|Default|GetPlayerActions)) _unitontile)
              (Actor|DestroyActor _unitontile))))
        (:then_1
          (bind _returnvalue (Game|SpawnActorfromClass "/Game/Blueprints/Core/Units/BP_Unit.BP_Unit_C" (Math|Transform|MakeTransform "0, 0, 0") "Undefined" "MultiplyWithRoot" 0 (Variables|Default|GetUnitType) 0))
          (Default|AddUnittoCombat (Variables|/Game/Blueprints/Core/Player/BP_PlayerActions.BP_PlayerActions_C|GetCombatSystem (Variables|Default|GetPlayerActions)) _returnvalue Index (Variables|Default|GetTeamIndex) (Variables|Default|GetUseAI)))))
    (else
      (goto _label))))