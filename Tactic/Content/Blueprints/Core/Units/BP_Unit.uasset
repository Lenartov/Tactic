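; BP_Unit is a grid-based unit actor that takes its stats, mesh and AnimBP from its unit type.
; It follows tile paths with a timeline that lerps transforms, hops on height changes and fires walk events, while its collision mesh matches the grid's tile shape.
; Spell hits change HP immediately, but hit or death reactions wait for the spell animation's tile-hit event.
; Hover and selection tint materials, and animation states go through AnimInstance messages.
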(event Custom|Event_FollowPath
  (params (Path :type Array%20of%20Int%20Point%20Structures))
  (if (> (Utilities|Array|Length Path) 0)
    (Variables|Default|SetCurrentPath Path)
    (Default|CallOnUnitStatedWalking self)
    (CallFunction|EventContinuetoFollowPath)))

(event Custom|Event_ContinueToFollowPath
  (bind _grid (Variables|Default|GetGrid))
  (bind _currentpath (Variables|Default|GetCurrentPath))
  (bind _timeline_unitmovement (Variables|Default|GetTimeline_UNitMovement))
  (bind _output (Utilities|Array|Get(acopy) _currentpath))
  (bind _gridtiles (Variables|/Game/Blueprints/Core/Grid/BP_Grid.BP_Grid_C|GetGridTiles _grid))
  (bind _value (Utilities|Map|Find _gridtiles _output))
  (bind _transform (Utilities|Struct|BreakS_TileData _value))
  (bind _location (Math|Transform|BreakTransform _transform))
  (if (> (Utilities|Array|Length (Variables|Default|GetCurrentPath)) 0)
    (CallFunction|SetAnimState "NewEnumerator1")
    (Variables|Default|SetPrevTransform (Transformation|GetActorTransform))
    (Variables|Default|SetNextTransform (Math|Transform|MakeTransform _location (Math|Rotator|FindLookatRotation (.Location (Math|Transform|BreakTransform (Variables|Default|GetPrevTransform))) _location)))
    (Components|Timeline|SetPlayRate _timeline_unitmovement (/ (Components|Timeline|GetTimelineLength _timeline_unitmovement) (Variables|Default|GetMoveDurationPerTile)))
    (bind (_direction _locationalpha _rotationalpha _jump) (Timeline|Timeline_UnitMovement PlayFromStart)
      (:Update
        (Transformation|SetActorLocationAndRotation (+ (Math|Vector|Lerp(Vector) (.Location (Math|Transform|BreakTransform (Variables|Default|GetPrevTransform))) (.Location (Math|Transform|BreakTransform (Variables|Default|GetNextTransform))) _locationalpha) (Math|Vector|MakeVector 0.0 0.0 (select (Math|Float|NearlyEqual(Float) (.Z (Math|Vector|BreakVector (.Location (Math|Transform|BreakTransform (Variables|Default|GetPrevTransform))))) (.Z (Math|Vector|BreakVector (.Location (Math|Transform|BreakTransform (Variables|Default|GetNextTransform))))) 5.0) 0.0 _jump))) (Math|Rotator|MakeRotator 0.0 0.0 (.Yaw (Math|Rotator|BreakRotator (Math|Rotator|Lerp(Rotator) (.Rotation (Math|Transform|BreakTransform (Variables|Default|GetPrevTransform))) (.Rotation (Math|Transform|BreakTransform (Variables|Default|GetNextTransform))) _rotationalpha true))))))
      (:Finished
        (Default|CallOnUnitReachedNewTile self (Utilities|Array|Get(acopy) (Variables|Default|GetCurrentPath)))
        (Utilities|Array|RemoveIndex (Variables|Default|GetCurrentPath))
        (CallFunction|EventContinuetoFollowPath)))
    (else
      (CallFunction|SetAnimState "NewEnumerator0")
      (Default|CallOnUnitFinishWalking self))))

(event Custom|DebugRespawnAfterFewSeconds
  (Utilities|FlowControl|Delay 2.0)
  (CallFunction|SetCurrentHP (.HPMax (Utilities|Struct|BreakS_UnitDataStats (.Stats (Utilities|Struct|BreakS_UnitData (Variables|Default|GetUnitData))))))
  (CallFunction|SetAnimState "NewEnumerator4"))

(event EventBeginPlay
  (CallFunction|SetAnimState "NewEnumerator0"))

(fn ConstructionScript
  (bind _data (CallFunction|GetDefaultUnitDatafromType (Variables|Default|GetUnitType)))
  (CallFunction|SetUnitData _data))

(fn UpdateVisualonHoverorSelected
  (Rendering|Material|SetVectorParameterValueonMaterials (Variables|Default|GetSkeletalMesh) "ColorMultiplier" (Math|Conversions|ToVector(LinearColor) (* (* (select (Variables|Default|GetIsSelected) "(R=0.161458,G=0.163529,B=0.645833,A=1.000000)" "(R=1.000000,G=1.000000,B=1.000000,A=1.000000)") (select (Variables|Default|GetIsHovered) 2.5 1.0)) (select (Variables|Default|GetIsSelected) 3.0 1.0)))))

(fn SetHovered
  (params (IsHovered :type Boolean))
  (Variables|Default|SetIsHovered IsHovered)
  (CallFunction|UpdateVisualonHoverorSelected))

(fn SetSelected
  (params (IsSelected :type Boolean))
  (Variables|Default|SetIsSelected IsSelected)
  (CallFunction|UpdateVisualonHoverorSelected))

(fn SetUnitData
  (params (Data :type S%20Unit%20Data%20Structure%20%28by%20ref%29))
  (bind _skeletalmesh (Variables|Default|GetSkeletalMesh))
  (bind _output_get (Variables|Default|SetUnitData Data))
  (Components|SkinnedMesh|SetSkinnedAssetandUpdate _skeletalmesh (.Mesh (Utilities|Struct|BreakS_UnitDataAssets (.Assets (Utilities|Struct|BreakS_UnitData _output_get)))) true)
  (Components|SkeletalMesh|SetAnimInstanceClass _skeletalmesh (.AnimBp (Utilities|Struct|BreakS_UnitDataAssets (.Assets (Utilities|Struct|BreakS_UnitData _output_get))))))

(fn SetAnimState
  (params (State :type E_UnitAnimState%20Enum :default "NewEnumerator0"))
  (Class|BPIUnitAnim|SetUnitAnimState(Message) (Components|SkeletalMesh|GetAnimInstance (Variables|Default|GetSkeletalMesh)) State))

(fn SetGrid
  (params (Grid :type BP%20Grid%20Object%20Reference))
  (bind _staticmeshcollision (Variables|Default|GetStaticMeshCollision))
  (bind _output_get (Variables|Default|SetGrid Grid))
  (Components|StaticMesh|SetStaticMesh _staticmeshcollision (.Mesh (Utilities|Struct|BreakS_GridData (Default|GetShapeData _output_get))))
  (Transformation|SetAbsolute (Variables|Default|GetStaticMeshCollision) false true true)
  (Transformation|SetWorldScale3D _staticmeshcollision (Math|Vector|MakeVector (.X (Math|Vector|BreakVector (/ (Variables|/Game/Blueprints/Core/Grid/BP_Grid.BP_Grid_C|GetTile%20Size (Variables|Default|GetGrid)) (.MeshSize (Utilities|Struct|BreakS_GridData (Default|GetShapeData _output_get)))))) (.Y (Math|Vector|BreakVector (/ (Variables|/Game/Blueprints/Core/Grid/BP_Grid.BP_Grid_C|GetTile%20Size (Variables|Default|GetGrid)) (.MeshSize (Utilities|Struct|BreakS_GridData (Default|GetShapeData _output_get)))))) (.Z (Math|Vector|BreakVector (Transformation|GetWorldScale (Variables|Default|GetStaticMeshCollision))))))
  (Transformation|SetWorldRotation (Variables|Default|GetStaticMeshCollision) (Default|GetRotationfromIndex Grid (Variables|Default|GetIndex)) false false))

(fn SetGridIndex
  (params (Index :type Int%20Point%20Structure))
  (Variables|Default|SetIndex Index)
  (Transformation|SetWorldRotation (Variables|Default|GetStaticMeshCollision) (Default|GetRotationfromIndex (Variables|Default|GetGrid) (Variables|Default|GetIndex)) false false))

(fn CastSpell
  (params (TargetIndex :type Int%20Point%20Structure))
  (bind _returnvalue (Transformation|GetActorLocation))
  (bind _grid (Variables|Default|GetGrid))
  (bind (_x _y) (Math|Vector|BreakVector _returnvalue))
  (bind _gridtiles (Variables|/Game/Blueprints/Core/Grid/BP_Grid.BP_Grid_C|GetGridTiles _grid))
  (bind _value (Utilities|Map|Find _gridtiles TargetIndex))
  (bind _transform (Utilities|Struct|BreakS_TileData _value))
  (bind _location (Math|Transform|BreakTransform _transform))
  (bind (_x_2 _y_2) (Math|Vector|BreakVector _location))
  (Transformation|SetActorRotation (Math|Rotator|FindLookatRotation (Math|Vector|MakeVector _x _y 0.0) (Math|Vector|MakeVector _x_2 _y_2 0.0)))
  (CallFunction|SetAnimState "NewEnumerator2"))

(fn ModifyCurrentHP
  (params (Modifier :type Integer))
  (CallFunction|SetCurrentHP (+ Modifier (.HPCurrent (Utilities|Struct|BreakS_UnitDataStats (.Stats (Utilities|Struct|BreakS_UnitData (Variables|Default|GetUnitData))))))))

(fn SetCurrentHP
  (params (HP :type Integer))
  (bind _structout (Utilities|Struct|SetmembersinS_UnitDataStats (.Stats (Utilities|Struct|BreakS_UnitData (Variables|Default|GetUnitData))) (Math|Integer|Clamp(Integer) HP 0 (.HPMax (Utilities|Struct|BreakS_UnitDataStats (.Stats (Utilities|Struct|BreakS_UnitData (Variables|Default|GetUnitData))))))))
  (Utilities|Struct|SetmembersinS_UnitData (Variables|Default|GetUnitData) _structout))

(fn UnitHitbySpell
  (params (SpellImpact :type S%20Spell%20Data%20Impact%20Real%20Structure) (SpellAnim :type BP%20Spell%20Anim%20Object%20Reference))
  (bind _hpmodifier (Utilities|Struct|BreakS_SpellDataImpactReal SpellImpact))
  (Utilities|Map|Add (Variables|Default|GetIncomingSpellImpacts) SpellAnim SpellImpact)
  (EventDispatchers|BindEventtoOnSpellAnimHitTile SpellAnim (EventDispatchers|CreateEvent :!event OnSpellAnimHitTile))
  (if (!= 0 _hpmodifier)
    (CallFunction|ModifyCurrentHP _hpmodifier)))

(fn OnSpellAnimHitTile
  (params (SpellAnim :type BP%20Spell%20Anim%20Object%20Reference) (Index :type Int%20Point%20Structure))
  (bind _incomingspellimpacts (Variables|Default|GetIncomingSpellImpacts))
  (bind (_value _returnvalue) (Utilities|Map|Find _incomingspellimpacts SpellAnim))
  (if (Class|KismetMathLibrary|EqualIntPointIntPoint Index (Variables|Default|GetIndex))
    (if _returnvalue
      (LocalVariables|SetSpellImpact _value)
      (Utilities|Map|Remove (Variables|Default|GetIncomingSpellImpacts) SpellAnim)
      (if (< (Utilities|Struct|BreakS_SpellDataImpactReal (LocalVariables|GetSpellImpact)) 0)
        (if (<= (.HPCurrent (Utilities|Struct|BreakS_UnitDataStats (.Stats (Utilities|Struct|BreakS_UnitData (Variables|Default|GetUnitData))))) 0)
          (if (Utilities|Enum|NotEqual(Enum) "NewEnumerator3" (CallFunction|GetAnimState))
            (CallFunction|SetAnimState "NewEnumerator3"))
          (else
            (CallFunction|SetAnimState "NewEnumerator5")))))))

(fn GetAnimState
  (bind _state (Class|BPIUnitAnim|GetUnitAnimState(Message) (Components|SkeletalMesh|GetAnimInstance (Variables|Default|GetSkeletalMesh))))
  (return _state))