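; Turn-based combat AI for the Ranger unit, extending a parent unit AI with its own choice of movement logic.
; It counts turns from combat start and flags when it casts a spell with a negative HP impact, clearing that flag each turn.
; GetUnitMovementLogic switches to an alternate movement mode only on odd turns after such a damaging cast, otherwise returning the first mode.
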(event EventBeginPlay
  (|CallParentFunction) ; This node is disabled and will not be called.\nDrag off pins to build functionality.
)

(event Collision|EventActorBeginOverlap
  (params (OtherActor :type Actor%20Object%20Reference)))

(event EventTick
  (params (DeltaSeconds :type Float%20%28single-precision%29)))

(event EventCastSpell
  (bind _data (CallFunction|GetSpellDatafromSpell (.Spell (Utilities|Struct|BreakS_UnitAISpellCastingData (Variables|Default|GetAISpellCasting)))))
  (Variables|Default|SetDamagedUnitThisTurn (or (< (.X (Utilities|Struct|BreakIntPoint (.MinMaxHPModifier (Utilities|Struct|BreakS_SpellDataImpact (.Impact (Utilities|Struct|BreakS_SpellData _data)))))) 0) (Variables|Default|GetDamagedUnitThisTurn)))
  (|CallParentFunction))

(fn ConstructionScript
  (|CallParentFunction))

(fn AIPlayTurn
  (Math|Integer|IncrementInt (Variables|Default|GetTurnCount)
    (:%20%20
      (Variables|Default|SetDamagedUnitThisTurn false)
      (|CallParentFunction))))

(fn GetUnitMovementLogic
  (return (select (or (CallFunction|IsIntEven (Variables|Default|GetTurnCount)) (not (Variables|Default|GetDamagedUnitThisTurn))) "NewEnumerator0" "NewEnumerator2")))

(fn AICombatStarted
  (Variables|Default|SetTurnCount 0)
  (|CallParentFunction))