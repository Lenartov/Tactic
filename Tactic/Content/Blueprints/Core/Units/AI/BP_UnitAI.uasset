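; Base unit AI that plays a combat turn as a fixed sequence of steps, with no decision, movement or casting logic in this graph.
; The chain runs from choosing a spell, moving and casting through choosing and moving to an end-turn location.
; A shared macro sets each state, broadcasts the change and waits a configurable delay.
; The final state hands control to CombatSystem's next unit.
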(event EventBeginPlay)

(event Collision|EventActorBeginOverlap
  (params (OtherActor :type Actor%20Object%20Reference)))

(event EventTick
  (params (DeltaSeconds :type Float%20%28single-precision%29)))

(event Custom|RunAILogic
  (Utilities|SetAIStatewithDelay "NewEnumerator1"
    (:Completed
      (CallFunction|DecideWhichSpelltoCast))))

(event Custom|DecideWhichSpellToCast_Done
  (CallFunction|MovetoSpellCastLocation))

(event Custom|CastSpell
  (Utilities|SetAIStatewithDelay "NewEnumerator4"
    (:Completed
      (CallFunction|CastSpellDone))))

(event Custom|MoveToEndTurnLocation_Done
  (Utilities|SetAIStatewithDelay "NewEnumerator7"
    (:Completed
      (CallFunction|AIEndTurn))))

(event Custom|DecideWhereToEndTurn
  (Utilities|SetAIStatewithDelay "NewEnumerator5"
    (:Completed
      (CallFunction|DecideWheretoEndTurnDone))))

(event Custom|MoveToEndTurnLocation
  (Utilities|SetAIStatewithDelay "NewEnumerator6"
    (:Completed
      (CallFunction|MovetoEndTurnLocationDone))))

(event Custom|DecideWhichSpellToCast
  (Utilities|SetAIStatewithDelay "NewEnumerator2"
    (:Completed
      (CallFunction|DecideWhichSpelltoCastDone))))

(event Custom|MoveToSpellCastLocation_Done
  (CallFunction|CastSpell))

(event Custom|CastSpell_Done
  (CallFunction|DecideWheretoEndTurn))

(event Custom|MoveToSpellCastLocation
  (Utilities|SetAIStatewithDelay "NewEnumerator3"
    (:Completed
      (CallFunction|MovetoSpellCastLocationDone))))

(event Custom|DecideWhereToEndTurn_Done
  (CallFunction|MovetoEndTurnLocation))

(fn ConstructionScript)

(fn AIPlayTurn
  (CallFunction|RunAILogic))

(fn AIEndTurn
  (Default|NextUnit (Variables|Default|GetCombatSystem)))