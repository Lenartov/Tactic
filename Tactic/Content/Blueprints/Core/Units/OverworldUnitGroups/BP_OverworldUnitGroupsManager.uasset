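; Manages overworld unit groups, turning contact between a non-encounter group and an encounter group into quick combat.
; Unit events drive groups: encounter members scatter around the mover's destination, others follow in a chain, and hover spreads group-wide during combat.
; Combat saves positions, disables uninvolved units and builds a random-sized grid shaped by the loaded level.
; Afterwards it destroys losers outside team 0, heals other combatants, restores positions and resumes encounter wandering.
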(event EventBeginPlay)

(event Collision|EventActorBeginOverlap
  (params (OtherActor :type Actor%20Object%20Reference)))

(event EventTick
  (params (DeltaSeconds :type Float%20%28single-precision%29)))

(fn ConstructionScript)

(fn AddUnittoGroup
  (params (Unit :type BP%20Unit%20Object%20Reference) (GroupID :type Integer))
  (if (!= GroupID (Variables|/Game/Blueprints/Core/Units/BP_Unit.BP_Unit_C|GetOverworldGroupID Unit))
    (CallFunction|RemoveUnitfromCurrentGroup Unit)
    (if (>= GroupID 0)
      (bind _output_get (Variables|Default|SetGroup (.Value (Utilities|Map|Find (Variables|Default|GetUnitGroups) GroupID))))
      (Utilities|Array|Add (.Units (Utilities|Struct|BreakS_OverworldUnitGroup _output_get)) Unit)
      (Utilities|Struct|SetmembersinS_OverworldUnitGroup (Variables|Default|GetGroup) GroupID)
      (Utilities|Map|Add (Variables|Default|GetUnitGroups) GroupID (Variables|Default|GetGroup))
      (Variables|/Game/Blueprints/Core/Units/BP_Unit.BP_Unit_C|SetOverworldGroupID Unit GroupID)
      (Game|BindEventtoOnDestroyed Unit (EventDispatchers|CreateEvent :!event OnUnitDestroyed))
      (EventDispatchers|BindEventtoOnUnitHoveredChanged Unit (EventDispatchers|CreateEvent :!event OnUNitHoveredChanged))
      (EventDispatchers|BindEventtoOnUnitStartedWalkinginOverworld Unit (EventDispatchers|CreateEvent :!event OnUNitStartedWalkinginOverworld))
      (EventDispatchers|BindEventtoOnUnitReachedUnitinOverworld Unit (EventDispatchers|CreateEvent :!event OnUnitReachedUnitinOverworld)))))

(fn RemoveUnitfromCurrentGroup
  (params (Unit :type BP%20Unit%20Object%20Reference))
  (bind _unitgroups (Variables|Default|GetUnitGroups))
  (if (>= (Variables|/Game/Blueprints/Core/Units/BP_Unit.BP_Unit_C|GetOverworldGroupID Unit) 0)
    (Variables|Default|SetGroup (.Value (Utilities|Map|Find (Variables|Default|GetUnitGroups) (Variables|/Game/Blueprints/Core/Units/BP_Unit.BP_Unit_C|GetOverworldGroupID Unit))))
    (Utilities|Array|RemoveItem (.Units (Utilities|Struct|BreakS_OverworldUnitGroup (Variables|Default|GetGroup))) Unit)
    (if (> (Utilities|Array|Length (.Units (Utilities|Struct|BreakS_OverworldUnitGroup (Variables|Default|GetGroup)))) 0)
      (Utilities|Map|Add _unitgroups (Variables|/Game/Blueprints/Core/Units/BP_Unit.BP_Unit_C|GetOverworldGroupID Unit) (Variables|Default|GetGroup))
      (else
        (Utilities|Map|Remove _unitgroups (Variables|/Game/Blueprints/Core/Units/BP_Unit.BP_Unit_C|GetOverworldGroupID Unit))))
    (Variables|/Game/Blueprints/Core/Units/BP_Unit.BP_Unit_C|SetOverworldGroupID Unit -999)
    (EventDispatchers|UnbindEventfromOnUnitHoveredChanged Unit (EventDispatchers|CreateEvent :!event OnUnitHoveredChanged))
    (EventDispatchers|UnbindEventfromOnUnitStartedWalkinginOverworld Unit (EventDispatchers|CreateEvent :!event OnUnitStartedWalkinginOverworld))
    (EventDispatchers|UnbindEventfromOnUnitReachedUnitinOverworld Unit (EventDispatchers|CreateEvent :!event OnUnitReachedUnitinOverworld))))

(fn OnUnitDestroyed
  (params (DestroyedActor :type Actor%20Object%20Reference))
  (bind _asbp_unit (Utilities|Casting|CastToBP_Unit DestroyedActor))
  (CallFunction|RemoveUnitfromCurrentGroup _asbp_unit))

(fn OnUnitHoveredChanged
  (params (Unit :type BP%20Unit%20Object%20Reference))
  (bind _overworldgroupid (Variables|/Game/Blueprints/Core/Units/BP_Unit.BP_Unit_C|GetOverworldGroupID Unit))
  (bind _unitgroups (Variables|Default|GetUnitGroups))
  (bind (_value _returnvalue) (Utilities|Map|Find _unitgroups _overworldgroupid))
  (if (Variables|/Game/Blueprints/Core/Combat/BP_CombatSystem.BP_CombatSystem_C|GetIsInCombat (Variables|Default|GetCombatSystem))
    (if _returnvalue
      (bind _output_get (Variables|Default|SetGroup _value))
      (for _array_element (.Units (Utilities|Struct|BreakS_OverworldUnitGroup _output_get))
        (bind _output_get_2 (LocalVariables|SetU _array_element))
        (if (!= _output_get_2 Unit)
          (EventDispatchers|UnbindEventfromOnUnitHoveredChanged (LocalVariables|GetU) (EventDispatchers|CreateEvent :!event OnUnitHoveredChanged))
          (Default|SetHovered (LocalVariables|GetU) (Variables|/Game/Blueprints/Core/Units/BP_Unit.BP_Unit_C|GetIsHovered Unit))
          (EventDispatchers|BindEventtoOnUnitHoveredChanged (LocalVariables|GetU) (EventDispatchers|CreateEvent :!event OnUnitHoveredChanged)))))))

(fn OnUnitStartedWalkinginOverworld
  (params (Unit :type BP%20Unit%20Object%20Reference))
  (if (.IsEncounter (Utilities|Struct|BreakS_OverworldUnitGroup (.Value (Utilities|Map|Find (Variables|Default|GetUnitGroups) (Variables|/Game/Blueprints/Core/Units/BP_Unit.BP_Unit_C|GetOverworldGroupID Unit)))))
    (for _array_element (.Units (Utilities|Struct|BreakS_OverworldUnitGroup (.Value (Utilities|Map|Find (Variables|Default|GetUnitGroups) (Variables|/Game/Blueprints/Core/Units/BP_Unit.BP_Unit_C|GetOverworldGroupID Unit)))))
      (bind _output_get (LocalVariables|SetU _array_element))
      (if (!= _output_get Unit)
        (EventDispatchers|UnbindEventfromOnUnitStartedWalkinginOverworld _output_get (EventDispatchers|CreateEvent :!event OnUnitStartedWalkinginOverworld))
        (bind _randomlocation (Default|GetRandomReachableinRadius (LocalVariables|GetU) (Variables|/Game/Blueprints/Core/Units/BP_Unit.BP_Unit_C|GetTargetLocationInOverworld Unit) "(X=100.000000,Y=400.000000)"))
        (Default|MoveUnitinOverworld (LocalVariables|GetU) _randomlocation 0 false)
        (EventDispatchers|BindEventtoOnUnitStartedWalkinginOverworld (LocalVariables|GetU) (EventDispatchers|CreateEvent :!event OnUnitStartedWalkinginOverworld))))
    (else
      (LocalVariables|SetPrevUnitInChain Unit)
      (for _array_element_2 (.Units (Utilities|Struct|BreakS_OverworldUnitGroup (.Value (Utilities|Map|Find (Variables|Default|GetUnitGroups) (Variables|/Game/Blueprints/Core/Units/BP_Unit.BP_Unit_C|GetOverworldGroupID Unit)))))
        (bind _output_get_2 (LocalVariables|SetU _array_element_2))
        (if (!= _output_get_2 Unit)
          (EventDispatchers|UnbindEventfromOnUnitStartedWalkinginOverworld (LocalVariables|GetU) (EventDispatchers|CreateEvent :!event OnUnitStartedWalkinginOverworld))
          (Default|MoveUnitinOverworld (LocalVariables|GetU) "0, 0, 0" (LocalVariables|GetPrevUnitInChain) false)
          (LocalVariables|SetPrevUnitInChain (LocalVariables|GetU))
          (EventDispatchers|BindEventtoOnUnitStartedWalkinginOverworld (LocalVariables|GetU) (EventDispatchers|CreateEvent :!event OnUnitStartedWalkinginOverworld)))))))

(fn SetGroupIsEncounter
  (params (IsEncounter :type Boolean) (GroupID :type Integer))
  (bind _unitgroups (Variables|Default|GetUnitGroups))
  (bind (_value _returnvalue) (Utilities|Map|Find _unitgroups GroupID))
  (if _returnvalue
    (bind _output_get (Variables|Default|SetGroup _value))
    (if (!= (.IsEncounter (Utilities|Struct|BreakS_OverworldUnitGroup _output_get)) IsEncounter)
      (Utilities|Struct|SetmembersinS_OverworldUnitGroup (Variables|Default|GetGroup) IsEncounter)
      (Utilities|Map|Add (Variables|Default|GetUnitGroups) GroupID (Variables|Default|GetGroup))
      (if (.IsEncounter (Utilities|Struct|BreakS_OverworldUnitGroup (Variables|Default|GetGroup)))
        (for _array_element (.Units (Utilities|Struct|BreakS_OverworldUnitGroup (Variables|Default|GetGroup)))
          (Default|StopMovingUnitinOverworld _array_element))
        (if (.IsEncounter (Utilities|Struct|BreakS_OverworldUnitGroup (Variables|Default|GetGroup)))
          (Default|MoveUnitinOverworld (Utilities|Array|Get(acopy) (.Units (Utilities|Struct|BreakS_OverworldUnitGroup (Variables|Default|GetGroup)))) "0, 0, 0" 0 true))))))

(fn SetCombatSystem
  (params (CombatSystem :type BP%20Combat%20System%20Object%20Reference))
  (bind _output_get (Variables|Default|SetCombatSystem CombatSystem))
  (EventDispatchers|BindEventtoOnCombatEnded _output_get (EventDispatchers|CreateEvent :!event OnCombatEnded)))

(fn OnUnitReachedUnitinOverworld
  (params (Unit :type BP%20Unit%20Object%20Reference))
  (bind _unitgroups (Variables|Default|GetUnitGroups))
  (bind _output_get (LocalVariables|SetGroup1 (.Value (Utilities|Map|Find _unitgroups (Variables|/Game/Blueprints/Core/Units/BP_Unit.BP_Unit_C|GetOverworldGroupID Unit)))))
  (bind _output_get_2 (LocalVariables|SetGroup2 (.Value (Utilities|Map|Find _unitgroups (Variables|/Game/Blueprints/Core/Units/BP_Unit.BP_Unit_C|GetOverworldGroupID (Variables|/Game/Blueprints/Core/Units/BP_Unit.BP_Unit_C|GetUnit%20to%20Follow Unit))))))
  (if (Math|Boolean|ANDBoolean (!= (.GroupID (Utilities|Struct|BreakS_OverworldUnitGroup _output_get)) (.GroupID (Utilities|Struct|BreakS_OverworldUnitGroup _output_get_2))) (not (.IsEncounter (Utilities|Struct|BreakS_OverworldUnitGroup _output_get))) (.IsEncounter (Utilities|Struct|BreakS_OverworldUnitGroup _output_get_2)))
    (CallFunction|TriggerEncounter (Utilities|Array|MakeArray (LocalVariables|GetGroup1) (LocalVariables|GetGroup2)))))

(fn TriggerEncounter
  (params (Groups :type Array%20of%20S%20Overworld%20Unit%20Group%20Structures))
  (if (not (Variables|/Game/Blueprints/Core/Combat/BP_CombatSystem.BP_CombatSystem_C|GetIsInCombat (Variables|Default|GetCombatSystem)))
    (Utilities|FlowControl|Sequence
      (:then_0
        (Utilities|Map|Clear (Variables|Default|GetUnitPositionsWhenCombatStarted))
        (bind _values (Utilities|Map|Values (Variables|Default|GetUnitGroups)))
        (for _array_element _values
          (for _array_element_2 (.Units (Utilities|Struct|BreakS_OverworldUnitGroup _array_element))
            (Utilities|Map|Add (Variables|Default|GetUnitPositionsWhenCombatStarted) _array_element_2 (Transformation|GetActorLocation _array_element_2))
            (if (not (Utilities|Array|ContainsItem Groups _array_element))
              (Default|DisableUnit _array_element_2)))))
      (:then_1
        (LocalVariables|SetGridData (Utilities|Struct|MakeS_QuickCombatGrid true (Transformation|GetActorLocation (Utilities|Array|Get(acopy) (.Units (Utilities|Struct|BreakS_OverworldUnitGroup (Utilities|Array|Get(acopy) Groups))))) "200.000000,200.000000,100.000000" (Utilities|Struct|MakeIntPoint (Math|Random|RandomIntegerinRange 10 20) (Math|Random|RandomIntegerinRange 10 20)) (CallFunction|GuessGridShapefromLoadedLevel)))
        (for _array_element_3 Groups
          (Utilities|Array|Add (LocalVariables|GetUnitTeams) (CallFunction|UnitsArraytoSpecialSet (.Units (Utilities|Struct|BreakS_OverworldUnitGroup _array_element_3))))
          (if (.IsEncounter (Utilities|Struct|BreakS_OverworldUnitGroup _array_element_3))
            (Utilities|Array|AppendArray (LocalVariables|GetControledByAI) (.Units (Utilities|Struct|BreakS_OverworldUnitGroup _array_element_3)))))
        (Default|QuickStartCombat (Variables|Default|GetCombatSystem) (LocalVariables|GetGridData) (Utilities|Struct|MakeS_QuickCombatUnitTeams (LocalVariables|GetUnitTeams) (LocalVariables|GetControledByAI) (Utilities|Map|MakeMap)) self)))))

(fn UnitsArraytoSpecialSet
  (params (Units :type Array%20of%20BP%20Unit%20Object%20References))
  (Utilities|Set|AddItems (LocalVariables|GetTempSet) Units)
  (return (Utilities|Struct|MakeS_UnitSet (LocalVariables|GetTempSet))))

(fn OnCombatEnded
  (bind _combatsystem (Variables|Default|GetCombatSystem))
  (bind _teamthatwonlastcombat (Variables|/Game/Blueprints/Core/Combat/BP_CombatSystem.BP_CombatSystem_C|GetTeamThatWonLastCombat _combatsystem))
  (if (== (Variables|/Game/Blueprints/Core/Combat/BP_CombatSystem.BP_CombatSystem_C|GetObjectThatStartedCombat (Variables|Default|GetCombatSystem)) self)
    (bind _keys (Utilities|Map|Keys (Variables|/Game/Blueprints/Core/Combat/BP_CombatSystem.BP_CombatSystem_C|GetUnitTeams (Variables|Default|GetCombatSystem))))
    (for _array_element _keys
      (LocalVariables|SetTeamIndex _array_element)
      (bind _result (Utilities|Set|ToArray (Utilities|Struct|BreakS_UnitSet (.Value (Utilities|Map|Find (Variables|/Game/Blueprints/Core/Combat/BP_CombatSystem.BP_CombatSystem_C|GetUnitTeams (Variables|Default|GetCombatSystem)) (LocalVariables|GetTeamIndex))))))
      (bind _output_get (LocalVariables|SetUnitsInTeam _result))
      (for _array_element_2 _output_get
        (bind _output_get_2 (LocalVariables|SetUnit _array_element_2))
        (Default|RemoveUnitfromCombat (Variables|Default|GetCombatSystem) _output_get_2)
        (if (Math|Boolean|ORBoolean (== (LocalVariables|GetTeamIndex) 0) (== (LocalVariables|GetTeamIndex) _teamthatwonlastcombat) (== _teamthatwonlastcombat -1))
          (Default|ResetHP (LocalVariables|GetUnit))
          (else
            (Actor|DestroyActor (LocalVariables|GetUnit))))))
    (bind _keys_2 (Utilities|Map|Keys (Variables|Default|GetUnitPositionsWhenCombatStarted)))
    (for _array_element_3 _keys_2
      (bind _output_get_3 (LocalVariables|SetUnit _array_element_3))
      (Utilities|IsValid _output_get_3
        (:Is%20Valid
          (Transformation|SetActorLocation (LocalVariables|GetUnit) (.Value (Utilities|Map|Find (Variables|Default|GetUnitPositionsWhenCombatStarted) (LocalVariables|GetUnit))) false false)
          (Default|EnableUnit (LocalVariables|GetUnit) "NewEnumerator1"))))
    (Utilities|Map|Clear (Variables|Default|GetUnitPositionsWhenCombatStarted))
    (bind _values (Utilities|Map|Values (Variables|Default|GetUnitGroups)))
    (for _array_element_4 _values
      (if (.IsEncounter (Utilities|Struct|BreakS_OverworldUnitGroup _array_element_4))
        (Default|MoveUnitinOverworld (Utilities|Array|Get(acopy) (.Units (Utilities|Struct|BreakS_OverworldUnitGroup _array_element_4))) "0, 0, 0" 0 true)))
    (Default|DestroyGrid (Variables|/Game/Blueprints/Core/Combat/BP_CombatSystem.BP_CombatSystem_C|GetGrid (Variables|Default|GetCombatSystem)))))

(fn GuessGridShapefromLoadedLevel
  (bind _enumvalue (|ForEachE_GridShape)
    (:LoopBody
      (Utilities|IsValid (Class|GameplayStatics|GetStreamingLevel (Utilities|String|StringToName (Utilities|String|Append "L_" (Utilities|String|EnumtoString _enumvalue))))
        (:Is%20Valid
          (if (Variables|/Script/Engine.LevelStreaming|GetbShouldBeVisible (Class|GameplayStatics|GetStreamingLevel (Utilities|String|StringToName (Utilities|String|Append "L_" (Utilities|String|EnumtoString _enumvalue)))))
            (return _enumvalue)))))
    (:then
      (return "NewEnumerator0"))))