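; Spell animation actor that launches a slime ball from the origin tile to the target tile.
; A timeline drives the interpolated location with a height offset, the scene scale and the opacity of three meshes, which the construction script tints in shades of green.
; Partway through playback a DoOnce reports a hit for each attacked tile index, and the timeline's end completes the spell animation.
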(event EventBeginPlay
  (|CallParentFunction) ; This node is disabled and will not be called.\nDrag off pins to build functionality.
)

(event Collision|EventActorBeginOverlap
  (params (OtherActor :type Actor%20Object%20Reference)))

(event EventTick
  (params (DeltaSeconds :type Float%20%28single-precision%29)))

(event EventPlaySpellAnim
  (Transformation|SetActorLocation (.Location (Math|Transform|BreakTransform (CallFunction|GetTileTransform (Variables|Default|GetOriginIndex)))) false false)
  (bind (_direction _opacity _scale _locationalpha _locationz) (Timeline|Timeline_SlimeBall PlayFromStart)
    (:Update
      (Transformation|SetActorLocation (+ (Math|Vector|Lerp(Vector) (.Location (Math|Transform|BreakTransform (CallFunction|GetTileTransform (Variables|Default|GetOriginIndex)))) (.Location (Math|Transform|BreakTransform (CallFunction|GetTileTransform (Variables|Default|GetTargetIndex)))) _locationalpha) (Math|Vector|MakeVector 0.0 0.0 _locationz)) false false)
      (Rendering|Material|SetScalarParameterValueonMaterials (Variables|Default|GetStaticMesh) "Opacity" _opacity)
      (Transformation|SetRelativeScale3D (Variables|Default|GetAnimScene) _scale)
      (if (>= (Components|Timeline|GetPlaybackPosition (Variables|Default|GetTimeline_SlimeBall)) 0.55)
        (Utilities|FlowControl|DoOnce false
          (:Completed
            (for _array_element (Variables|Default|GetAttackedIndexes)
              (Default|CallOnSpellAnimHitTile self _array_element))))))
    (:Finished
      (CallFunction|EventCompleteSpellAnim))))

(fn ConstructionScript
  (|CallParentFunction)
  (Rendering|Material|SetVectorParameterValueonMaterials (Variables|Default|GetStaticMesh) "Color" (Math|Conversions|ToVector(LinearColor) "(R=0.337123,G=0.895833,B=0.321940,A=1.000000)"))
  (Rendering|Material|SetVectorParameterValueonMaterials (Variables|Default|GetStaticMesh1) "Color" (Math|Conversions|ToVector(LinearColor) "(R=0.111437,G=0.822917,B=0.205758,A=1.000000)"))
  (Rendering|Material|SetVectorParameterValueonMaterials (Variables|Default|GetStaticMesh2) "Color" (Math|Conversions|ToVector(LinearColor) "(R=0.048055,G=0.796875,B=0.065521,A=1.000000)")))