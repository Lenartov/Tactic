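; Spell animation actor for a heal spell, shown as six green-tinted meshes on the target tile.
; PlaySpellAnim moves the actor to the target tile, then a timeline drives the scene's yaw and scale and the meshes' material opacity.
; Shortly into the timeline, a DoOnce-gated call signals the tile hit, and the timeline's end completes the spell animation.
; The construction script sets the green shades on the mesh materials.
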(event EventBeginPlay
  (|CallParentFunction) ; This node is disabled and will not be called.\nDrag off pins to build functionality.
)

(event Collision|EventActorBeginOverlap
  (params (OtherActor :type Actor%20Object%20Reference)))

(event EventTick
  (params (DeltaSeconds :type Float%20%28single-precision%29)))

(event EventPlaySpellAnim
  (bind _animscene (Variables|Default|GetAnimScene))
  (Transformation|SetActorLocation (.Location (Math|Transform|BreakTransform (CallFunction|GetTileTransform (Variables|Default|GetTargetIndex)))) false false)
  (bind (_direction _opacity _scale _rotation) (Timeline|Timeline_Heal PlayFromStart)
    (:Update
      (Transformation|SetRelativeRotation _animscene (Math|Rotator|MakeRotator 0.0 0.0 _rotation) false false)
      (Transformation|SetRelativeScale3D _animscene _scale)
      (Rendering|Material|SetScalarParameterValueonMaterials (Variables|Default|GetStaticMesh1) "Opacity" _opacity)
      (if (>= (Components|Timeline|GetPlaybackPosition (Variables|Default|GetTimeline_Heal)) 0.2)
        (Utilities|FlowControl|DoOnce false
          (:Completed
            (Default|CallOnSpellAnimHitTile self (Variables|Default|GetTargetIndex))))))
    (:Finished
      (CallFunction|EventCompleteSpellAnim))))

(fn ConstructionScript
  (|CallParentFunction)
  (Rendering|Material|SetVectorParameterValueonMaterials (Variables|Default|GetStaticMesh) "Color" (Math|Conversions|ToVector(LinearColor) "(R=0.437170,G=1.000000,B=0.421875,A=1.000000)"))
  (Rendering|Material|SetVectorParameterValueonMaterials (Variables|Default|GetStaticMesh1) "Color" (Math|Conversions|ToVector(LinearColor) "(R=0.135417,G=1.000000,B=0.250035,A=1.000000)"))
  (Rendering|Material|SetVectorParameterValueonMaterials (Variables|Default|GetStaticMesh2) "Color" (Math|Conversions|ToVector(LinearColor) "(R=0.060304,G=1.000000,B=0.082222,A=1.000000)"))
  (Rendering|Material|SetVectorParameterValueonMaterials (Variables|Default|GetStaticMesh3) "Color" (Math|Conversions|ToVector(LinearColor) "(R=0.437170,G=1.000000,B=0.421875,A=1.000000)"))
  (Rendering|Material|SetVectorParameterValueonMaterials (Variables|Default|GetStaticMesh4) "Color" (Math|Conversions|ToVector(LinearColor) "(R=0.135417,G=1.000000,B=0.250035,A=1.000000)"))
  (Rendering|Material|SetVectorParameterValueonMaterials (Variables|Default|GetStaticMesh5) "Color" (Math|Conversions|ToVector(LinearColor) "(R=0.060304,G=1.000000,B=0.082222,A=1.000000)")))