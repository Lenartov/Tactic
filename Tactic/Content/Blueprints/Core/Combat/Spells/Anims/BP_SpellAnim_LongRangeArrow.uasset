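; Spell animation actor that flies a long-range arrow from an origin tile to a target tile.
; PlaySpellAnim places it on the origin tile, facing the target via a look-at rotation built from the two tiles' 2D coordinates.
; Timeline_SwordThrow then lerps its location with an added height offset, while driving the pitch and scale of SceneScaleRotation.
; When the timeline finishes, it calls EventCompleteSpellAnim.
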(event EventBeginPlay
  (|CallParentFunction) ; This node is disabled and will not be called.\nDrag off pins to build functionality.
)

(event Collision|EventActorBeginOverlap
  (params (OtherActor :type Actor%20Object%20Reference)))

(event EventTick
  (params (DeltaSeconds :type Float%20%28single-precision%29)))

(event EventPlaySpellAnim
  (Transformation|SetActorLocationAndRotation (.Location (Math|Transform|BreakTransform (CallFunction|GetTileTransform (Variables|Default|GetOriginIndex)))) (Math|Rotator|FindLookatRotation (Math|Conversions|ToVector(Vector2D) (Math|Conversions|ToVector2D(IntPoint) (Variables|Default|GetOriginIndex))) (Math|Conversions|ToVector(Vector2D) (Math|Conversions|ToVector2D(IntPoint) (Variables|Default|GetTargetIndex)))))
  (bind (_direction _locationalpha _locationz _rotationy _scale) (Timeline|Timeline_SwordThrow PlayFromStart)
    (:Update
      (Transformation|SetActorLocation (+ (Math|Vector|Lerp(Vector) (.Location (Math|Transform|BreakTransform (CallFunction|GetTileTransform (Variables|Default|GetOriginIndex)))) (.Location (Math|Transform|BreakTransform (CallFunction|GetTileTransform (Variables|Default|GetTargetIndex)))) _locationalpha) (Math|Vector|MakeVector 0.0 0.0 _locationz)) false false)
      (Transformation|SetRelativeRotation (Variables|Default|GetSceneScaleRotation) (Math|Rotator|MakeRotator 0.0 _rotationy 0.0) false false)
      (Transformation|SetRelativeScale3D (Variables|Default|GetSceneScaleRotation) (Math|Conversions|ToVector(Float) _scale)))
    (:Finished
      (CallFunction|EventCompleteSpellAnim))))

(fn ConstructionScript
  (|CallParentFunction))