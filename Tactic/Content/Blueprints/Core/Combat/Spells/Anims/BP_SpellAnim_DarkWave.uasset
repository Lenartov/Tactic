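; BP_SpellAnim_DarkWave is the visual animation actor for the Dark Wave spell.
; When played, it moves to the target tile, and a timeline scales its AnimScene component while driving the Opacity material parameter on three static meshes.
; The construction script tints each mesh a slightly different shade of purple, and timeline completion calls the shape-anim completion handler.
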(event EventBeginPlay
  (|CallParentFunction) ; This node is disabled and will not be called.\nDrag off pins to build functionality.
)

(event Collision|EventActorBeginOverlap
  (params (OtherActor :type Actor%20Object%20Reference)))

(event EventTick
  (params (DeltaSeconds :type Float%20%28single-precision%29)))

(event EventPlaySpellAnim
  (Transformation|SetActorLocation (.Location (Math|Transform|BreakTransform (CallFunction|GetTileTransform (Variables|Default|GetTargetIndex)))) false false)
  (bind (_direction _opacity _scale) (Timeline|Timeline_DarkWave PlayFromStart)
    (:Update
      (Transformation|SetRelativeScale3D (Variables|Default|GetAnimScene) _scale)
      (Rendering|Material|SetScalarParameterValueonMaterials (Variables|Default|GetStaticMesh1) "Opacity" _opacity))
    (:Finished
      (CallFunction|OnShapeAnimComplited))))

(fn ConstructionScript
  (|CallParentFunction)
  (Rendering|Material|SetVectorParameterValueonMaterials (Variables|Default|GetStaticMesh) "Color" (Math|Conversions|ToVector(LinearColor) "(R=0.621296,G=0.281250,B=1.000000,A=1.000000)"))
  (Rendering|Material|SetVectorParameterValueonMaterials (Variables|Default|GetStaticMesh1) "Color" (Math|Conversions|ToVector(LinearColor) "(R=0.572549,G=0.125490,B=1.000000,A=1.000000)"))
  (Rendering|Material|SetVectorParameterValueonMaterials (Variables|Default|GetStaticMesh2) "Color" (Math|Conversions|ToVector(LinearColor) "(R=0.509804,G=0.000000,B=1.000000,A=1.000000)")))