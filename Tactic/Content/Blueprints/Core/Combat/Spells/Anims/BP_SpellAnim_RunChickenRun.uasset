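; Spell animation actor for Run Chicken Run that shows the spell's icon over the targeted tile.
; On play, it moves to the target tile's location and sets the icon on its widget component's image.
; A timeline drives the widget's height, draw size and opacity, fires the tile-hit callback once shortly after starting, and completes the spell animation when finished.
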(event EventBeginPlay
  (|CallParentFunction) ; This node is disabled and will not be called.\nDrag off pins to build functionality.
)

(event Collision|EventActorBeginOverlap
  (params (OtherActor :type Actor%20Object%20Reference)))

(event EventTick
  (params (DeltaSeconds :type Float%20%28single-precision%29)))

(event EventPlaySpellAnim
  (bind _widget (Variables|Default|GetWidget))
  (Transformation|SetActorLocation (.Location (Math|Transform|BreakTransform (CallFunction|GetTileTransform (Variables|Default|GetTargetIndex)))) false false)
  (bind _output_get (Variables|Default|SetImage (.AsW%20Image (Utilities|Casting|CastToW_Image (UserInterface|GetUserWidgetObject (Variables|Default|GetWidget))))))
  (Appearance|SetBrushfromTexture (Variables|/Game/Blueprints/Core/Combat/Spells/Anims/Components/W_Image.W_Image_C|GetImageComponent _output_get) "/Game/Blueprints/Core/Combat/Spells/Anims/Assets/Icon_RunChickenRun_NoBackground.Icon_RunChickenRun_NoBackground" false)
  (bind (_direction _locationz _drawsize _opacity) (Timeline|Timeline_RunChickenRun PlayFromStart)
    (:Update
      (Transformation|SetRelativeLocation _widget (Math|Vector|MakeVector 0.0 0.0 _locationz) false false)
      (Class|WidgetComponent|SetDrawSize _widget (Math|Vector2D|MakeVector2D _drawsize _drawsize))
      (Widget|SetRenderOpacity (Variables|Default|GetImage) _opacity)
      (if (>= (Components|Timeline|GetPlaybackPosition (Variables|Default|GetTimeline_RunChickenRun)) 0.2)
        (Utilities|FlowControl|DoOnce false
          (:Completed
            (Default|CallOnSpellAnimHitTile self (Variables|Default|GetTargetIndex))))))
    (:Finished
      (CallFunction|EventCompleteSpellAnim))))

(fn ConstructionScript
  (|CallParentFunction))