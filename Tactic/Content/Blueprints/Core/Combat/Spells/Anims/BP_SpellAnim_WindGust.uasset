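; Spell animation actor for the Wind Gust spell, playing gusts that blow outward from the target tile to the other attacked tiles.
; After a short delay it reports a hit on the target tile, then spawns a BP_AnimWindGust toward each remaining attacked tile, growing in scale at a random play rate.
; Each gust reports a hit on its tile when it finishes, and the spell animation completes once none remain.
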(event Custom|CustomEvent
  (params (AnimShape :type BP%20Anim%20Wind%20Gust%20Object%20Reference))
  (bind _index (Variables|/Game/Blueprints/Core/Combat/Spells/Anims/Components/BP_AnimWindGust.BP_AnimWindGust_C|GetIndex AnimShape))
  (bind _attackedindexes (Variables|Default|GetAttackedIndexes))
  (Default|CallOnSpellAnimHitTile self _index)
  (Utilities|Array|RemoveItem _attackedindexes _index)
  (if (<= (Utilities|Array|Length _attackedindexes) 0)
    (CallFunction|EventCompleteSpellAnim)))

(event EventBeginPlay
  (|CallParentFunction) ; This node is disabled and will not be called.\nDrag off pins to build functionality.
)

(event Collision|EventActorBeginOverlap
  (params (OtherActor :type Actor%20Object%20Reference)))

(event EventTick
  (params (DeltaSeconds :type Float%20%28single-precision%29)))

(event EventPlaySpellAnim
  (bind _targetindex (Variables|Default|GetTargetIndex))
  (bind _targetindex_2 (Variables|Default|GetTargetIndex))
  (bind _transform (CallFunction|GetTileTransform _targetindex))
  (Utilities|FlowControl|Delay 0.1)
  (Default|CallOnSpellAnimHitTile self _targetindex_2)
  (Utilities|Array|RemoveItem (Variables|Default|GetAttackedIndexes) _targetindex_2)
  (for _array_element (Variables|Default|GetAttackedIndexes)
    (bind _returnvalue (Game|SpawnActorfromClass "/Game/Blueprints/Core/Combat/Spells/Anims/Components/BP_AnimWindGust.BP_AnimWindGust_C" (Math|Transform|MakeTransform "0, 0, 0" "0, 0, 0" "1.000000,1.000000,1.000000") "AlwaysSpawn" "MultiplyWithRoot" 0 (Math|Transform|MakeTransform (.location _transform) (Math|Rotator|FindLookatRotation (.location _transform) (.location (CallFunction|GetTileTransform _array_element))) "0.500000,0.500000,0.500000") (Math|Transform|MakeTransform (.location (CallFunction|GetTileTransform _array_element)) (Math|Rotator|FindLookatRotation (.location _transform) (.location (CallFunction|GetTileTransform _array_element))) "1.200000,1.200000,1.200000") (Math|Random|RandomFloatinRange 0.5 1.5) _array_element 0))
    (EventDispatchers|BindEventtoOnShapeAnimComplited _returnvalue (delegate Custom|CustomEvent))))

(fn ConstructionScript
  (|CallParentFunction))