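; Short-lived wind gust visual for spell animations, moving its mesh from an origin transform to a target transform.
; Construction gives two material slots translucent green dynamic materials with randomized brightness.
; On BeginPlay, a rate-adjusted timeline lerps the actor transform and feeds an opacity track to a material scalar.
; It signals shape completion once at 0.35 seconds of playback, then destroys itself shortly after the timeline finishes.
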(event EventBeginPlay
  (Components|Timeline|SetPlayRate (Variables|Default|GetTimeline_PlayAnim) (Variables|Default|GetPlayRate))
  (bind (_direction _alphatransform _opacity) (Timeline|Timeline_PlayAnim PlayFromStart)
    (:Update
      (Transformation|SetActorTransform (Math|Transform|Lerp(Transform) (Variables|Default|GetOriginTransform) (Variables|Default|GetTargetTransform) _alphatransform))
      (Rendering|Material|SetScalarParameterValueonMaterials (Variables|Default|GetStaticMesh) "None" _opacity)
      (if (>= (Components|Timeline|GetPlaybackPosition (Variables|Default|GetTimeline_PlayAnim)) 0.35)
        (Utilities|FlowControl|DoOnce false
          (:Completed
            (Default|CallOnShapeAnimComplited self)))))
    (:Finished
      (Utilities|FlowControl|Delay 0.5)
      (Actor|DestroyActor))))

(fn ConstructionScript
  (bind _returnvalue (Rendering|Material|CreateDynamicMaterialInstance (Variables|Default|GetStaticMesh) 0 "/Game/Art/Materials/M_ColorTranslucent.M_ColorTranslucent" "None" :!class /Script/Engine.PrimitiveComponent))
  (Rendering|Material|SetVectorParameterValue _returnvalue "Color" (* "(R=0.093416,G=0.442708,B=0.165165,A=1.000000)" (Math|Random|RandomFloatinRange 0.8 1.5)) :!class /Script/Engine.MaterialInstanceDynamic)
  (bind _returnvalue_2 (Rendering|Material|CreateDynamicMaterialInstance (Variables|Default|GetStaticMesh) 1 "/Game/Art/Materials/M_ColorTranslucent.M_ColorTranslucent" "None" :!class /Script/Engine.PrimitiveComponent))
  (Rendering|Material|SetVectorParameterValue _returnvalue_2 "Color" (* "(R=0.196370,G=0.661458,B=0.291905,A=1.000000)" (Math|Random|RandomFloatinRange 0.8 1.5)) :!class /Script/Engine.MaterialInstanceDynamic))