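; BP_AnimShape is a spell animation actor that flies a configurable mesh from an origin transform to a target transform.
; On BeginPlay it applies the mesh, material and color, then plays a timeline at a set play rate.
; The timeline lerps the transform and adds a fixed lift plus an animated height offset.
; When finished, it fires a completion dispatcher and destroys itself after a short delay.
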(event EventBeginPlay
  (bind _staticmesh (Variables|Default|GetStaticMesh))
  (Components|StaticMesh|SetStaticMesh _staticmesh (Variables|Default|GetMesh))
  (Rendering|Material|SetMaterial _staticmesh 0 (Variables|Default|GetMaterial))
  (Rendering|Material|SetVectorParameterValueonMaterials _staticmesh "Color" (Math|Conversions|ToVector(LinearColor) (Variables|Default|GetColor)))
  (Components|Timeline|SetPlayRate (Variables|Default|GetTimeline_PlayAnim) (Variables|Default|GetPlayRate))
  (bind (_direction _alphatransform _hightoffset) (Timeline|Timeline_PlayAnim PlayFromStart)
    (:Update
      (Transformation|SetActorTransform (Math|Transform|MakeTransform (+ (.Location (Math|Transform|BreakTransform (Math|Transform|Lerp(Transform) (Variables|Default|GetOriginTransform) (Variables|Default|GetTargetTransform) _alphatransform))) "0.000000,0.000000,100.000000" (Math|Vector|MakeVector 0.0 0.0 _hightoffset)) (.Rotation (Math|Transform|BreakTransform (Math|Transform|Lerp(Transform) (Variables|Default|GetOriginTransform) (Variables|Default|GetTargetTransform) _alphatransform))) (.Scale (Math|Transform|BreakTransform (Math|Transform|Lerp(Transform) (Variables|Default|GetOriginTransform) (Variables|Default|GetTargetTransform) _alphatransform))))))
    (:Finished
      (Default|CallOnShapeAnimComplited self)
      (Utilities|FlowControl|Delay 0.4)
      (Actor|DestroyActor))))

(fn ConstructionScript)