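; BP_SpellAnim is a transient actor that plays a spell's visual effect on the combat grid and destroys itself when finished.
; On BeginPlay it spawns a BP_AnimShape per target tile, using the grid's shape mesh and material to animate from a shrunken origin-tile transform to that target.
; Each shape gets randomized red brightness and play rate for variation.
; Only the first shape's completion fires the spell-complete dispatcher, even if others are still animating.
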(event Custom|Event_PlaySpellAnim
  (bind _grid (Variables|Default|GetGrid))
  (bind _originindex (Variables|Default|GetOriginIndex))
  (bind _returnvalue (Default|GetShapeData _grid))
  (bind _transform (CallFunction|GetTileTransform _originindex))
  (bind (_meshsize _mesh _meshmaterial) (Utilities|Struct|BreakS_GridData _returnvalue))
  (bind (_location _rotation) (Math|Transform|BreakTransform _transform))
  (for (_array_element _array_index) (Variables|Default|GetTargetIndexes)
    (bind _returnvalue_2 (Game|SpawnActorfromClass "/Game/Blueprints/Core/Combat/Spells/Components/BP_AnimShape.BP_AnimShape_C" (Math|Transform|MakeTransform "0, 0, 0") "AlwaysSpawn" "MultiplyWithRoot" 0 _mesh _meshmaterial (* "(R=1.000000,G=0.000000,B=0.000000,A=1.000000)" (Math|Random|RandomFloatinRange 0.5 1.5)) (Math|Transform|MakeTransform _location _rotation "0.100000,0.100000,0.100000") (CallFunction|GetTileTransform _array_element) (Math|Random|RandomFloatinRange 1.1 1.6) 0))
    (if (== _array_index 0)
      (EventDispatchers|BindEventtoOnShapeAnimComplited _returnvalue_2 (delegate Custom|OnShapeAnimComplited)))))

(event Custom|OnShapeAnimComplited
  (params (AnimShape :type BP%20Anim%20Shape%20Object%20Reference))
  (CallFunction|EventCompleteSpellAnim))

(event Custom|Event_CompleteSpellAnim
  (Default|CallONSpellAnimComplited self)
  (Actor|DestroyActor))

(event EventBeginPlay
  (CallFunction|EventPlaySpellAnim))

(fn ConstructionScript)

(fn GetTileTransform
  (params (Index :type Int%20Point%20Structure))
  (return (.Transform (Utilities|Struct|BreakS_TileData (.Value (Utilities|Map|Find (Variables|/Game/Blueprints/Core/Grid/BP_Grid.BP_Grid_C|GetGridTiles (Variables|Default|GetGrid)) Index))))))