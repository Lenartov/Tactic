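; BP_GridVisual is the actor that renders a tile grid through two child instanced-mesh actors: a flat walkable-tile overlay and a 3D tactical view.
; Tile updates re-add instances in both layers, stretching tactical meshes vertically relative to the grid's lowest Z.
; Tactical mode toggles that layer's visibility and query collision, hides actors tagged NotTactical, and lazily rebuilds tactical tiles when flagged stale.
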(event EventBeginPlay
  (Actor|Tick|SetActorTickEnabled false))

(fn ConstructionScript)

(fn InitGridVisual
  (params (Grid :type BP%20Grid%20Object%20Reference))
  (Variables|Default|SetGrid Grid)
  (bind _asbp_grid_mesh_inst (Utilities|Casting|CastToBP_GridMeshInst (Variables|/Script/Engine.ChildActorComponent|GetChildActor (Variables|Default|GetChildActorGridMeshInst))))
  (Variables|Default|SetGridMeshInst _asbp_grid_mesh_inst)
  (bind _asbp_grid_mesh_inst_2 (Utilities|Casting|CastToBP_GridMeshInst (Variables|/Script/Engine.ChildActorComponent|GetChildActor (Variables|Default|GetChildActorGridMeshTacticInst))))
  (Variables|Default|SetGridMeshInstTactic _asbp_grid_mesh_inst_2)
  (Default|InitGridMeshInst (Variables|Default|GetGridMeshInst) (.FlatMesh (Utilities|Struct|BreakS_GridData (Default|GetShapeData (Variables|Default|GetGrid)))) (.FlatMaterial (Utilities|Struct|BreakS_GridData (Default|GetShapeData (Variables|Default|GetGrid)))) "NoCollision" false)
  (Default|InitGridMeshInst (Variables|Default|GetGridMeshInstTactic) (.Mesh (Utilities|Struct|BreakS_GridData (Default|GetShapeData (Variables|Default|GetGrid)))) (.MeshMaterial (Utilities|Struct|BreakS_GridData (Default|GetShapeData (Variables|Default|GetGrid)))) "NoCollision" true)
  (Transformation|SetActorLocation "0, 0, 0" false false)
  (CallFunction|SetOffsetfromGround (Variables|Default|GetOffset))
  (CallFunction|SetGridLowestZ 999999.0)
  (CallFunction|SetIsTactic (Variables|Default|GetIs%20Tactical)))

(fn SetOffsetfromGround
  (params (Offset :type Float%20%28double-precision%29))
  (Variables|Default|SetOffset Offset)
  (Transformation|SetRelativeLocation (Variables|Default|GetChildActorGridMeshInst) (Math|Vector|MakeVector 0.0 0.0 (Variables|Default|GetOffset)) false false))

(fn DestroyGridVisual
  (bind _gridmeshinsttactic (Variables|Default|GetGridMeshInstTactic))
  (bind _gridmeshinst (Variables|Default|GetGridMeshInst))
  (Utilities|FlowControl|Sequence
    (:then_0
      (Utilities|IsValid _gridmeshinst
        (:Is%20Valid
          (Default|ClearInstances _gridmeshinst))))
    (:then_1
      (Utilities|IsValid _gridmeshinsttactic
        (:Is%20Valid
          (Default|ClearInstances _gridmeshinsttactic))))
    (:then_2
      (CallFunction|SetGridLowestZ 999999.0))))

(fn UpdateTileVisual
  (params (Data :type S%20Tile%20Data%20Structure))
  (Utilities|FlowControl|Sequence
    (:then_0
      (Default|RemoveInstance (Variables|Default|GetGridMeshInst) (.index Data))
      (if (CallFunction|IsTileWalkable (.tiletype Data))
        (Default|AddInstance (Variables|Default|GetGridMeshInst) (.transform Data) (.index Data) (.states Data) (.tiletype Data))))
    (:then_1
      (CallFunction|UpdateTileTacticVisual Data))))

(fn UpdateTileTacticVisual
  (params (Data :type S%20Tile%20Data%20Structure))
  (bind _grid (Variables|Default|GetGrid))
  (bind _transform (Utilities|Struct|BreakS_TileData Data))
  (bind (_location _rotation _scale) (Math|Transform|BreakTransform (.transform Data)))
  (bind _returnvalue (Default|GetShapeData _grid))
  (bind _location_2 (Math|Transform|BreakTransform _transform))
  (bind _z (Math|Vector|BreakVector _location_2))
  (Utilities|FlowControl|Sequence
    (:then_0
      (if (< _z (Variables|Default|GetGridLowestZ))
        (CallFunction|SetGridLowestZ _z)))
    (:then_1
      (if (Variables|Default|GetIs%20Tactical)
        (Default|RemoveInstance (Variables|Default|GetGridMeshInstTactic) (.index Data))
        (if (Utilities|Enum|NotEqual(Enum) (.tiletype Data) "NewEnumerator0")
          (Default|AddInstance (Variables|Default|GetGridMeshInstTactic) (Math|Transform|MakeTransform _location _rotation (Math|Vector|MakeVector (.x _scale) (.y _scale) (/ (+ (- (.Z (Math|Vector|BreakVector (.Location (Math|Transform|BreakTransform (.Transform (Utilities|Struct|BreakS_TileData Data)))))) (Variables|Default|GetGridLowestZ)) (.z (.meshsize _returnvalue))) (.z (.meshsize _returnvalue))))) (.index Data) (.states Data) (.tiletype Data)))
        (else
          (Variables|Default|SetNeedToRegenTacticOnNextEnabl true))))))

(fn SetGridLowestZ
  (params (GridLowestZ :type Float%20%28double-precision%29))
  (Variables|Default|SetGridLowestZ GridLowestZ)
  (Variables|Default|SetNeedToRegenTacticOnNextEnabl true))

(fn SetIsTactic
  (params (IsTactical :type Boolean))
  (bind _grid (Variables|Default|GetGrid))
  (bind _gridmeshinsttactic (Variables|Default|GetGridMeshInstTactic))
  (Variables|Default|SetIs%20Tactical IsTactical)
  (Development|SetHiddeninGame (Variables|Default|GetChildActorGridMeshTacticInst) (not (Variables|Default|GetIs%20Tactical)) false)
  (bind _outactors (Actor|GetAllActorswithTag "NotTactical"))
  (for _array_element _outactors
    (Rendering|SetActorHiddenInGame _array_element (Variables|Default|GetIs%20Tactical)))
  (Utilities|FlowControl|Sequence
    (:then_0
      (if (and (Variables|Default|GetIs%20Tactical) (Variables|Default|GetNeedToRegenTacticOnNextEnabl))
        (Variables|Default|SetNeedToRegenTacticOnNextEnabl false)
        (Utilities|IsValid _grid
          (:Is%20Valid
            (bind _values (Utilities|Map|Values (Variables|/Game/Blueprints/Core/Grid/BP_Grid.BP_Grid_C|GetGridTiles _grid)))
            (for _array_element_2 _values
              (CallFunction|UpdateTileTacticVisual _array_element_2))))))
    (:then_1
      (Utilities|IsValid _gridmeshinsttactic
        (:Is%20Valid
          (Collision|SetCollisionEnabled (Variables|/Game/Blueprints/Core/Grid/Utilities/BP_GridMeshInst.BP_GridMeshInst_C|GetInstancedStaticMesh _gridmeshinsttactic) (select IsTactical "QueryOnly" "NoCollision")))))))