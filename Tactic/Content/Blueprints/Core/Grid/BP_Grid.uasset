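; Grid actor that builds a square, triangle or hex tile grid on construction and owns its tile data, with child actors for visuals and pathfinding.
; Sphere traces snap tile heights to the ground and take tile types from BP_GridModifier actors, with hexes using doubled-row indices.
; Tile and state edits update the visual and fire notifications, with a reverse state-to-index map for lookups.
; Helpers convert cursor or world positions to tile indices.
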(fn ConstructionScript
  (Variables|Default|SetGridVisual (.AsBP%20Grid%20Visual (Utilities|Casting|CastToBP_GridVisual (Variables|/Script/Engine.ChildActorComponent|GetChildActor (Variables|Default|GetChildActorGridVisual)))))
  (bind _output_get (Variables|Default|SetPathfinding (.AsBP%20Grid%20Pathfinding (Utilities|Casting|CastToBP_GridPathfinding (Variables|/Script/Engine.ChildActorComponent|GetChildActor (Variables|Default|GetChildActorPathfinding))))))
  (Variables|/Game/Blueprints/Core/Grid/BP_GridPathfinding.BP_GridPathfinding_C|SetGrid _output_get self)
  (CallFunction|SpawnGrid (Transformation|GetActorLocation) (Variables|Default|GetTile%20Size) (Variables|Default|GetTile%20Count) (Variables|Default|GetShape) true))

(fn SpawnGrid
  (params (Center :type Vector) (TileScale :type Vector) (TileCount :type Int%20Point%20Structure) (Shape :type E_GridShape%20Enum :default "NewEnumerator3") (UseEnvironment :type Boolean))
  (bind (_center _gridbottomleftloc) (CallFunction|CalculateCenterandBottomLeft))
  (Variables|Default|SetCenter Center)
  (Variables|Default|SetTile%20Size TileScale)
  (Variables|Default|SetShape Shape)
  (Variables|Default|SetTile%20Count TileCount)
  (Utilities|FlowControl|Sequence
    (:then_0
      (CallFunction|DestroyGrid)
      (Default|InitGridVisual (Variables|Default|GetGridVisual) self)
      (Variables|Default|SetCenter _center)
      (Variables|Default|SetGridBottomLeftLoc _gridbottomleftloc)
      (for _index (range 0 (- (.x (Variables|Default|GetTile%20Count)) 1))
        (LocalVariables|SetX _index)
        (if (Utilities|Enum|NotEqual(Enum) (Variables|Default|GetShape) "NewEnumerator2")
          (for _index_2 (range 0 (- (.y (Variables|Default|GetTile%20Count)) 1))
            (LocalVariables|SetY _index_2)
            (Variables|Default|SetIndex (Utilities|Struct|MakeIntPoint (LocalVariables|GetX) (LocalVariables|GetY)))
            (LocalVariables|SetTileTransform (Math|Transform|MakeTransform (CallFunction|GetLocationfromIndex (Variables|Default|GetIndex)) (CallFunction|GetRotationfromIndex (Variables|Default|GetIndex)) (CallFunction|GetTileScale)))
            (if UseEnvironment
              (bind (_outlocation _tiletype) (CallFunction|TraceforGround (.location (LocalVariables|GetTileTransform))))
              (CallFunction|AddGridTile (Utilities|Struct|MakeS_TileData (Variables|Default|GetIndex) _tiletype (Math|Transform|MakeTransform _outlocation (.rotation (LocalVariables|GetTileTransform)) (.scale (LocalVariables|GetTileTransform))) "NewEnumerator0" 0))
              (else
                (CallFunction|AddGridTile (Utilities|Struct|MakeS_TileData (Variables|Default|GetIndex) "NewEnumerator1" (LocalVariables|GetTileTransform) "NewEnumerator0" 0)))))
          (else
            (for _index_3 (range (Math|Integer|SelectInt 0 1 (CallFunction|IsIntEven (LocalVariables|GetX))) (- (* (.y (Variables|Default|GetTile%20Count)) 2.0) 1))
              (LocalVariables|SetY _index_3)
              (Utilities|FlowControl|Sequence
                (:then_0
                  (Variables|Default|SetIndex (Utilities|Struct|MakeIntPoint (LocalVariables|GetX) (LocalVariables|GetY)))
                  (LocalVariables|SetTileTransform (Math|Transform|MakeTransform (CallFunction|GetLocationfromIndex (Variables|Default|GetIndex)) (CallFunction|GetRotationfromIndex (Variables|Default|GetIndex)) (CallFunction|GetTileScale)))
                  (if UseEnvironment
                    (bind (_outlocation_2 _tiletype_2) (CallFunction|TraceforGround (.location (LocalVariables|GetTileTransform))))
                    (CallFunction|AddGridTile (Utilities|Struct|MakeS_TileData (Variables|Default|GetIndex) _tiletype_2 (Math|Transform|MakeTransform _outlocation_2 (.rotation (LocalVariables|GetTileTransform)) (.scale (LocalVariables|GetTileTransform))) "NewEnumerator0" 0))
                    (else
                      (CallFunction|AddGridTile (Utilities|Struct|MakeS_TileData (Variables|Default|GetIndex) "NewEnumerator1" (LocalVariables|GetTileTransform) "NewEnumerator0" 0)))))
                (:then_1
                  (Math|Integer|IncrementInt _index_3))))))))
    (:then_1
      (Default|CallOnGridGenerated))))

(fn GetShapeData
  (return (CallFunction|GetShapeData (Variables|Default|GetShape))))

(fn DestroyGrid
  (Utilities|Map|Clear (Variables|Default|GetGridTiles))
  (Default|DestroyGridVisual (Variables|Default|GetGridVisual))
  (Default|CallOnGridDestroy))

(fn CalculateCenterandBottomLeft
  (bind _tile_count (Variables|Default|GetTile%20Count))
  (bind _tile_size (Variables|Default|GetTile%20Size))
  (bind _center (Variables|Default|GetCenter))
  (bind _center_2 (Variables|Default|GetCenter))
  (bind _tile_size_2 (Variables|Default|GetTile%20Size))
  (switch Utilities|FlowControl|Switch|SwitchonE_GridShape (Variables|Default|GetShape)
    (:NewEnumerator0
      (bind _output_get (LocalVariables|SetC (CallFunction|SnapVectortoVector (Variables|Default|GetCenter) (Variables|Default|GetTile%20Size))))
      (return _output_get (- (Variables|Default|GetCenter) (* (/ (- (Variables|Default|GetTile%20Count) (Math|Vector2D|MakeVector2D (Math|Conversions|ToFloat(Integer) (Math|Integer|SelectInt 0 1 (CallFunction|IsIntEven (.x _tile_count)))) (Math|Conversions|ToFloat(Integer) (Math|Integer|SelectInt 0 1 (CallFunction|IsIntEven (.y _tile_count)))))) "2.000000,2.000000,1.000000") (Variables|Default|GetTile%20Size)))))
    (:NewEnumerator1
      (bind _output_get_2 (LocalVariables|SetC (CallFunction|SnapVectortoVector _center (* (Variables|Default|GetTile%20Size) "2.000000,1.000000,1.000000"))))
      (return _output_get_2 (- _center (CallFunction|SnapVectortoVector (* (/ (- (Variables|Default|GetTile%20Count) (Math|Vector2D|MakeVector2D 1.0 1.0)) "2.000000,4.000000,1.000000") _tile_size) (* _tile_size "2.000000,1.000000,1.000000")))))
    (:NewEnumerator2
      (bind _output_get_3 (LocalVariables|SetC (CallFunction|SnapVectortoVector _center_2 (* (Variables|Default|GetTile%20Size) "1.500000,1.000000,1.000000"))))
      (return _output_get_3 (- _center_2 (CallFunction|SnapVectortoVector (* (/ (Math|Conversions|ToVector2D(IntPoint) (Variables|Default|GetTile%20Count)) "3.000000,2.000000,1.000000") _tile_size_2) (* _tile_size_2 "1.500000,1.000000,1.000000")))))))

(fn GetRotationfromIndex
  (params (GridIndex :type Int%20Point%20Structure))
  (bind _index (Variables|Default|GetIndex))
  (if (Utilities|Enum|Equal(Enum) "NewEnumerator1" (Variables|Default|GetShape))
    (return (Math|Rotator|MakeRotator 0.0 0.0 (+ (Math|Float|SelectFloat 1.8e+02 0.0 (CallFunction|IsIntEven (.x _index))) (Math|Float|SelectFloat 1.8e+02 0.0 (CallFunction|IsIntEven (.y _index))))))
    (else
      (return "0, 0, 0"))))

(fn GetLocationfromIndex
  (params (Index :type Int%20Point%20Structure))
  (return (+ (Variables|Default|GetGridBottomLeftLoc) (* (Variables|Default|GetTile%20Size) (* Index (Utilities|Select :Index (Variables|Default|GetShape) :NewEnumerator3 "" :NewEnumerator0 "(X=1.000000,Y=1.000000)" :NewEnumerator1 "(X=1.000000,Y=0.500000)" :NewEnumerator2 "(X=0.750000,Y=0.500000)"))))))

(fn TraceforGround
  (params (Location :type Vector))
  (bind _output_get (LocalVariables|SetRadius (/ (.x (Variables|Default|GetTile%20Size)) (Math|Float|SelectFloat 5.0 3.0 (Utilities|Enum|Equal(Enum) (Variables|Default|GetShape) "NewEnumerator1")))))
  (bind _outhits (Collision|MultiSphereTraceByChannel (+ Location "0.000000,0.000000,1000.000000") (- Location "0.000000,0.000000,1000.000000") _output_get "TraceTypeQuery3" false 0 "None" true "(R=1.000000,G=0.000000,B=0.000000,A=1.000000)" "(R=0.000000,G=1.000000,B=0.000000,A=1.000000)" 1.0))
  (if (> (Utilities|Array|Length _outhits) 0)
    (LocalVariables|SetIsHeightFound false)
    (LocalVariables|SetRetType "NewEnumerator1")
    (for _array_element _outhits
      (bind _asbp_grid_modifier (Utilities|Casting|CastToBP_GridModifier (.HitActor (Collision|BreakHitResult _array_element)))
        (:then
          (if (Utilities|Enum|Equal(Enum) (Variables|/Game/Blueprints/Core/Grid/BP_GridModifier.BP_GridModifier_C|GetType _asbp_grid_modifier) "NewEnumerator3")
            (if true
              (LocalVariables|SetRetType (Variables|/Game/Blueprints/Core/Grid/BP_GridModifier.BP_GridModifier_C|GetType _asbp_grid_modifier) :!label _label)
              (if (Variables|/Game/Blueprints/Core/Grid/BP_GridModifier.BP_GridModifier_C|GetUseForTileHight _asbp_grid_modifier)
                (LocalVariables|SetIsHeightFound true)
                (LocalVariables|SetRetZ (Math|Float|SnapToGrid(Float) (- (.Z (Math|Vector|BreakVector (.Location (Collision|BreakHitResult _array_element)))) (LocalVariables|GetRadius)) (.z (Variables|Default|GetTile%20Size))) :!label _label_2)))
            (elif true
              (goto _label))))
        (:CastFailed
          (if (not (LocalVariables|GetIsHeightFound))
            (goto _label_2)))))
    (return (Math|Vector|MakeVector (.x Location) (.y Location) (LocalVariables|GetRetZ)) (LocalVariables|GetRetType))
    (else
      (return Location "NewEnumerator0"))))

(fn AddGridTile
  (params (Data :type S%20Tile%20Data%20Structure))
  (if (Utilities|Enum|Equal(Enum) (.tiletype Data) "NewEnumerator3")
    (if true
      (Utilities|Map|Add (Variables|Default|GetGridTiles) (.index Data) Data :!label _label)
      (Default|UpdateTileVisual (Variables|Default|GetGridVisual) Data)
      (Default|CallOnTileDataUpdate (.index Data)))
    (elif true
      (goto _label))))

(fn GetCursoreLocation
  (params (PlayerIndex :type Integer))
  (bind _returnvalue (Game|GetPlayerController PlayerIndex))
  (bind _center (Variables|Default|GetCenter))
  (bind (_hitresult _returnvalue_2) (Game|Player|GetHitResultUnderCursorbyChannel _returnvalue "TraceTypeQuery3" false))
  (bind (_worldlocation _worlddirection) (Game|Player|ConvertMouseLocationToWorldSpace _returnvalue))
  (bind _returnvalue_3 (Class|KismetMathLibrary|MakePlanefromPointandNormal _center "0.000000,0.000000,1.000000"))
  (bind (_hitresult_2 _returnvalue_4) (Game|Player|GetHitResultUnderCursorbyChannel _returnvalue "TraceTypeQuery4" false))
  (bind _returnvalue_5 (* _worlddirection 999999.0))
  (bind _returnvalue_6 (+ _worldlocation _returnvalue_5))
  (bind (_t _intersection _returnvalue_7) (Class|KismetMathLibrary|LinePlaneIntersection _worldlocation _returnvalue_6 _returnvalue_3))
  (if _returnvalue_4
    (return (.Location (Collision|BreakHitResult _hitresult_2)))
    (elif _returnvalue_2
      (return (.Location (Collision|BreakHitResult _hitresult)))
      (elif _returnvalue_7
        (return _intersection)
        (else
          (return "-99999.000000,-99999.000000,-99999.000000"))))))

(fn GetTileIndexfromWorldLoc
  (params (Location :type Vector))
  (LocalVariables|SetLocationOnGrid (- Location (Variables|Default|GetGridBottomLeftLoc)))
  (switch Utilities|FlowControl|Switch|SwitchonE_GridShape (Variables|Default|GetShape)
    (:NewEnumerator3
      (return (Utilities|Struct|MakeIntPoint -1 -1)))
    (:NewEnumerator0
      (bind _output_get (LocalVariables|SetSnapedLocationOnGrid (Math|Conversions|ToVector2D(Vector) (CallFunction|SnapVectortoVector (LocalVariables|GetLocationOnGrid) (Variables|Default|GetTile%20Size)))))
      (return (Class|KismetMathLibrary|ToIntPoint(Vector2D) (/ _output_get (Variables|Default|GetTile%20Size)))))
    (:NewEnumerator1
      (bind _output_get_2 (LocalVariables|SetSnapedLocationOnGrid (Math|Conversions|ToVector2D(Vector) (CallFunction|SnapVectortoVector (LocalVariables|GetLocationOnGrid) (/ (Variables|Default|GetTile%20Size) "1.000000,2.000000,1.000000")))))
      (return (Class|KismetMathLibrary|ToIntPoint(Vector2D) (* (/ _output_get_2 (Variables|Default|GetTile%20Size)) "(X=1.000000,Y=2.000000)"))))
    (:NewEnumerator2
      (bind _output_get_3 (LocalVariables|SetSnapedLocationOnGrid (Math|Conversions|ToVector2D(Vector) (CallFunction|SnapVectortoVector (* (LocalVariables|GetLocationOnGrid) "1.000000,2.000000,1.000000") (* (Variables|Default|GetTile%20Size) "0.750000,0.250000,1.000000")))))
      (bind _output_get_4 (LocalVariables|SetTempIndex (/ _output_get_3 (* (Variables|Default|GetTile%20Size) "(X=0.750000,Y=1.000000)"))))
      (if (CallFunction|IsFloatEven (.x _output_get_4))
        (return (Utilities|Struct|MakeIntPoint (Math|Float|Truncate (.x (LocalVariables|GetTempIndex))) (* (Math|Float|Round (/ (.y (LocalVariables|GetTempIndex)) 2.0)) 2)))
        (else
          (return (Utilities|Struct|MakeIntPoint (Math|Float|Truncate (.x (LocalVariables|GetTempIndex))) (+ (* (Math|Float|Floor (/ (.y (LocalVariables|GetTempIndex)) 2.0)) 2) 1))))))))

(fn GetTileIndexUnderCursor
  (params (PlayerIndex :type Integer))
  (bind _location (CallFunction|GetCursoreLocation PlayerIndex))
  (bind _index (CallFunction|GetTileIndexfromWorldLoc _location))
  (return _index))

(fn AddState
  (params (Index :type Int%20Point%20Structure) (State :type E_TileState%20Enum :default "NewEnumerator0"))
  (bind _gridtiles (Variables|Default|GetGridTiles))
  (bind (_value _returnvalue) (Utilities|Map|Find _gridtiles Index))
  (if _returnvalue
    (bind _output_get (LocalVariables|SetData _value))
    (bind _returnvalue_2 (Utilities|Array|AddUnique (.states _output_get) State))
    (if (>= _returnvalue_2 0)
      (Utilities|Map|Add (Variables|Default|GetGridTiles) (.index (LocalVariables|GetData)) (LocalVariables|GetData))
      (bind _indexes (CallFunction|GetAllTileswithState State))
      (Utilities|Array|Add _indexes Index)
      (Utilities|Map|Add (Variables|Default|GetTileStatesToIndexes) State (Utilities|Struct|MakeS_IntPointArray _indexes))
      (Default|UpdateTileVisual (Variables|Default|GetGridVisual) (LocalVariables|GetData))
      (Default|CallOnTileStateUpdated (.index (LocalVariables|GetData))))))

(fn RemoveState
  (params (Index :type Int%20Point%20Structure) (State :type E_TileState%20Enum :default "NewEnumerator0"))
  (bind _gridtiles (Variables|Default|GetGridTiles))
  (bind (_value _returnvalue) (Utilities|Map|Find _gridtiles Index))
  (if _returnvalue
    (bind _output_get (LocalVariables|SetData _value))
    (bind _returnvalue_2 (Utilities|Array|RemoveItem (.states _output_get) State))
    (if _returnvalue_2
      (Utilities|Map|Add (Variables|Default|GetGridTiles) (.index (LocalVariables|GetData)) (LocalVariables|GetData))
      (bind _indexes (CallFunction|GetAllTileswithState State))
      (Utilities|Array|RemoveItem _indexes Index)
      (Utilities|Map|Add (Variables|Default|GetTileStatesToIndexes) State (Utilities|Struct|MakeS_IntPointArray _indexes))
      (Default|UpdateTileVisual (Variables|Default|GetGridVisual) (LocalVariables|GetData))
      (Default|CallOnTileStateUpdated Index))))

(fn IsIndexValid
  (params (Index :type Int%20Point%20Structure))
  (return (Utilities|Map|Contains (Variables|Default|GetGridTiles) Index)))

(fn GetTileScale
  (return (/ (Variables|Default|GetTile%20Size) (.MeshSize (Utilities|Struct|BreakS_GridData (CallFunction|GetShapeData))))))

(fn RemoveTile
  (params (Index :type Int%20Point%20Structure))
  (bind _returnvalue (Utilities|Map|Remove (Variables|Default|GetGridTiles) Index))
  (if _returnvalue
    (Default|UpdateTileVisual (Variables|Default|GetGridVisual) (Utilities|Struct|MakeS_TileData Index "NewEnumerator0" "0.000000,0.000000,0.000000|0.000000,0.000000,0.000000|1.000000,1.000000,1.000000" "NewEnumerator0" 0))
    (Default|CallOnTileDataUpdate Index)))

(fn GetAllTileswithState
  (params (State :type E_TileState%20Enum :default "NewEnumerator0"))
  (return (.intpointarray (.Value (Utilities|Map|Find (Variables|Default|GetTileStatesToIndexes) State)))))

(fn ClearStatesfromTiles
  (params (State :type E_TileState%20Enum :default "NewEnumerator0"))
  (bind _indexes (CallFunction|GetAllTileswithState State))
  (for _array_element _indexes
    (CallFunction|RemoveState _array_element State)))

(fn IsTileWalkable
  (params (Index :type Int%20Point%20Structure))
  (return (CallFunction|IsTileWalkable (.TileType (Utilities|Struct|BreakS_TileData (.Value (Utilities|Map|Find (Variables|Default|GetGridTiles) Index)))))))