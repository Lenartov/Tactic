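; Grid visual actor that draws tiles through one InstancedStaticMesh, with mesh, material, color and collision set at init.
; A parallel InstanceIndexes array maps grid indices to instances, so tiles can be replaced, removed or cleared.
; Each added tile resolves its states by priority (Selected, Hovered, IsNeighborn) into a highlight color and fill flag, written to per-instance custom data for the material.
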(event EventBeginPlay
  (Actor|Tick|SetActorTickEnabled false))

(fn ConstructionScript)

(fn AddInstance
  (params (Transform :type Transform) (Index :type Int%20Point%20Structure%20%28by%20ref%29) (States :type Array%20of%20E_TileState%20Enums :default "NewEnumerator0"))
  (bind _instancedstaticmesh (Variables|Default|GetInstancedStaticMesh))
  (CallFunction|RemoveInstance Index)
  (Components|InstancedStaticMesh|AddInstance (Variables|Default|GetInstancedStaticMesh) Transform false)
  (bind _returnvalue (Utilities|Array|Add (Variables|Default|GetInstanceIndexes) Index))
  (LocalVariables|SetI _returnvalue)
  (bind (_color _isfilled) (CallFunction|GetColorfromStates States))
  (Components|InstancedStaticMesh|SetCustomDataValue _instancedstaticmesh (LocalVariables|GetI) 0 (.R (Math|Color|BreakColor _color)) false)
  (Components|InstancedStaticMesh|SetCustomDataValue _instancedstaticmesh (LocalVariables|GetI) 1 (.G (Math|Color|BreakColor _color)) false)
  (Components|InstancedStaticMesh|SetCustomDataValue _instancedstaticmesh (LocalVariables|GetI) 2 (.B (Math|Color|BreakColor _color)) false)
  (Components|InstancedStaticMesh|SetCustomDataValue _instancedstaticmesh (LocalVariables|GetI) 3 _isfilled false))

(fn RemoveInstance
  (params (Index :type Int%20Point%20Structure%20%28by%20ref%29))
  (if (Utilities|Array|ContainsItem (Variables|Default|GetInstanceIndexes) Index)
    (Class|InstancedStaticMeshComponent|RemoveInstance (Variables|Default|GetInstancedStaticMesh) (Utilities|Array|FindItem (Variables|Default|GetInstanceIndexes) Index))
    (Utilities|Array|RemoveItem (Variables|Default|GetInstanceIndexes) Index)))

(fn ClearInstances
  (Components|InstancedStaticMesh|ClearInstances (Variables|Default|GetInstancedStaticMesh))
  (Utilities|Array|Clear (Variables|Default|GetInstanceIndexes)))

(fn InitGridMeshInst
  (params (Mesh :type Static%20Mesh%20Object%20Reference) (Material :type Material%20Interface%20Object%20Reference) (Color :type Linear%20Color%20Structure) (Collision :type ECollisionEnabled%20Enum :default "NoCollision"))
  (bind _instancedstaticmesh (Variables|Default|GetInstancedStaticMesh))
  (Components|StaticMesh|SetStaticMesh _instancedstaticmesh Mesh)
  (Rendering|Material|SetMaterial _instancedstaticmesh 0 Material)
  (Rendering|Material|SetVectorParameterValueonMaterials _instancedstaticmesh "None" (Math|Conversions|ToVector(LinearColor) Color))
  (Collision|SetCollisionEnabled _instancedstaticmesh Collision))

(fn GetColorfromStates
  (params (States :type Array%20of%20E_TileState%20Enums :default "NewEnumerator0"))
  (if (Utilities|Array|IsEmpty States)
    (return "" 0.0)
    (else
      (for _array_element (Utilities|Array|MakeArray "NewEnumerator2" "NewEnumerator1" "NewEnumerator3")
        (if (Utilities|Array|ContainsItem States _array_element)
          (return (Utilities|Select :Index _array_element :NewEnumerator0 "" :NewEnumerator1 "(R=0.992711,G=1.000000,B=0.005208,A=1.000000)" :NewEnumerator2 "(R=0.401042,G=0.138907,B=0.018799,A=1.000000)" :NewEnumerator3 "(R=0.962132,G=0.338542,B=1.000000,A=1.000000)") 1.0)))
      (return "" 0.0))))