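; Combat scenario actor that quick-starts a grid battle on BeginPlay and returns to the main menu when the combat it started ends.
; Outside play, its construction script centers and spawns the grid on the actor, then maps placed units to tiles by their locations.
; Separate helpers, not called here, build teams by parsing "Team" numbers from unit names and assign all but the first team to AI.
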(event Custom|OnCombatEnded
  (if (== (Variables|/Game/Blueprints/Core/Combat/BP_CombatSystem.BP_CombatSystem_C|GetObjectThatStartedCombat (Variables|Default|GetCombatSystem)) self)
    (Game|OpenLevel(byName) "L_MainMenu")))

(event EventBeginPlay
  (EventDispatchers|BindEventtoOnCombatEnded (Variables|Default|GetCombatSystem) (delegate Custom|OnCombatEnded))
  (Default|QuickStartCombat (Variables|Default|GetCombatSystem) (Variables|Default|GetGridData) (Variables|Default|GetUnitsData) self))

(fn ConstructionScript
  (if (not (CallFunction|IsinGame))
    (Utilities|Struct|SetmembersinS_QuickCombatGrid (Variables|Default|GetGridData) (Transformation|GetActorLocation))
    (CallFunction|SpawnGrid)
    (CallFunction|BuildDesiredGridBaseonUnitLocations)))

(fn BuildTeamsBaseonUnitsName
  (bind _outactors (Actor|GetAllActorsOfClass "/Game/Blueprints/Core/Units/BP_Unit.BP_Unit_C"))
  (for _array_element _outactors
    (bind _output_get (LocalVariables|SetUnit _array_element))
    (bind _output_get_2 (LocalVariables|SetTeamIndex (Math|Conversions|ToInteger(Byte) (.LeftS (Utilities|String|Split (.RightS (Utilities|String|Split (Utilities|GetDisplayName _output_get) "Team")) "_")))))
    (if (< (Utilities|Array|Length (LocalVariables|GetUnitsTeams)) (+ _output_get_2 1))
      (Utilities|Array|Resize (LocalVariables|GetUnitsTeams) (+ _output_get_2 1)))
    (Utilities|Set|Add (Utilities|Struct|BreakS_UnitSet (Utilities|Array|Get(acopy) (LocalVariables|GetUnitsTeams) (LocalVariables|GetTeamIndex))) (LocalVariables|GetUnit)))
  (Utilities|Array|RemoveItem :TargetArray (LocalVariables|GetUnitsTeams))
  (Utilities|Struct|SetmembersinS_QuickCombatUnitTeams (Variables|Default|GetUnitsData) (LocalVariables|GetUnitsTeams)))

(fn BuildAIListBaseonTeamIndexes
  (for (_array_element _array_index) (.UnitTeams (Utilities|Struct|BreakS_QuickCombatUnitTeams (Variables|Default|GetUnitsData)))
    (if (!= _array_index 0)
      (bind _result (Utilities|Set|ToArray (Utilities|Struct|BreakS_UnitSet _array_element)))
      (Utilities|Array|AppendArray (LocalVariables|GetAIs) _result)))
  (Utilities|Struct|SetmembersinS_QuickCombatUnitTeams (Variables|Default|GetUnitsData) (LocalVariables|GetAIs)))

(fn BuildDesiredGridBaseonUnitLocations
  (for _array_element (.UnitTeams (Utilities|Struct|BreakS_QuickCombatUnitTeams (Variables|Default|GetUnitsData)))
    (bind _result (Utilities|Set|ToArray (Utilities|Struct|BreakS_UnitSet _array_element)))
    (for _array_element_2 _result
      (bind _index (Default|GetTileIndexfromWorldLoc (Variables|/Game/Blueprints/Core/Combat/BP_CombatSystem.BP_CombatSystem_C|GetGrid (Variables|Default|GetCombatSystem)) (Transformation|GetActorLocation _array_element_2)))
      (Utilities|Map|Add (LocalVariables|GetDesiredIndexes) _array_element_2 _index)))
  (Utilities|Struct|SetmembersinS_QuickCombatUnitTeams (Variables|Default|GetUnitsData) (LocalVariables|GetDesiredIndexes)))

(fn SpawnGrid
  (bind _combatsystem (Variables|Default|GetCombatSystem))
  (bind _griddata (Variables|Default|GetGridData))
  (bind (_generategridbeforestartingcombat _centerlocation _tilesize _tilecount _shape _useenvironment) (Utilities|Struct|BreakS_QuickCombatGrid _griddata))
  (bind _grid (Variables|/Game/Blueprints/Core/Combat/BP_CombatSystem.BP_CombatSystem_C|GetGrid _combatsystem))
  (Utilities|IsValid _combatsystem
    (:Is%20Valid
      (Utilities|IsValid _grid
        (:Is%20Valid
          (Default|SpawnGrid _grid _centerlocation _tilesize _tilecount _shape _useenvironment))))))