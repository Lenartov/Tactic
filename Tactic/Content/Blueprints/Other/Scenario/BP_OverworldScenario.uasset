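; Overworld scenario Blueprint that sets up the map's unit groups and adds the back-to-main-menu widget.
; On BeginPlay, after a brief delay, it sets each unit's context and registers the stored UnitGroups, with their encounter flags, in OverworldUnitGroupManager.
; BuildUnitGroupsBaseOnUnitNames, not called in this graph, rebuilds that map from all BP_Units, parsing group IDs after "Group" in display names and treating "_AI" as an encounter.
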(event EventBeginPlay
  (bind _returnvalue (UserInterface|CreateWidget "/Game/Blueprints/Other/MainMenu/W_BackToMainMenu.W_BackToMainMenu_C"))
  (UserInterface|Viewport|AddtoViewport _returnvalue 0)
  (Utilities|FlowControl|Delay 0.1)
  (bind _values (Utilities|Map|Values (Variables|Default|GetUnitGroups)))
  (for _array_element _values
    (for _array_element_2 (.Units (Utilities|Struct|BreakS_OverworldUnitGroup _array_element))
      (Default|SetContext _array_element_2 "NewEnumerator1")
      (Default|AddUnittoGroup (Variables|Default|GetOverworldUnitGroupManager) _array_element_2 (.GroupID (Utilities|Struct|BreakS_OverworldUnitGroup _array_element))))
    (Default|SetGroupIsEncounter (Variables|Default|GetOverworldUnitGroupManager) (.IsEncounter (Utilities|Struct|BreakS_OverworldUnitGroup _array_element)) (.GroupID (Utilities|Struct|BreakS_OverworldUnitGroup _array_element)))))

(fn ConstructionScript)

(fn BuildUnitGroupsBaseonUnitNames
  (Utilities|Map|Clear (Variables|Default|GetUnitGroups))
  (bind _outactors (Actor|GetAllActorsOfClass "/Game/Blueprints/Core/Units/BP_Unit.BP_Unit_C"))
  (for _array_element _outactors
    (bind _output_get (LocalVariables|SetUnit _array_element))
    (if (.ReturnValue (Utilities|String|Split (.RightS (Utilities|String|Split (Utilities|GetDisplayName _output_get) "Group")) "_"))
      (LocalVariables|SetGroupID (Math|Conversions|ToInteger(Byte) (.LeftS (Utilities|String|Split (.RightS (Utilities|String|Split (Utilities|GetDisplayName _output_get) "Group")) "_"))))
      (else
        (LocalVariables|SetGroupID (Math|Conversions|ToInteger(Byte) (.RightS (Utilities|String|Split (Utilities|GetDisplayName _output_get) "Group"))))))
    (LocalVariables|SetIsEncounter (Utilities|String|Contains (Utilities|GetDisplayName (LocalVariables|GetUnit)) "_AI"))
    (bind _output_get_2 (LocalVariables|SetGroup (.Value (Utilities|Map|Find (Variables|Default|GetUnitGroups) (LocalVariables|GetGroupID)))))
    (bind _structout (Utilities|Struct|SetmembersinS_OverworldUnitGroup _output_get_2 (LocalVariables|GetGroupID) (LocalVariables|GetIsEncounter)))
    (Utilities|Array|AddUnique (.Units (Utilities|Struct|BreakS_OverworldUnitGroup _structout)) (LocalVariables|GetUnit))
    (Utilities|Map|Add (Variables|Default|GetUnitGroups) (LocalVariables|GetGroupID) (LocalVariables|GetGroup))))